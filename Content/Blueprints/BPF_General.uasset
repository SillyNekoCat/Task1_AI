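; General Blueprint function library, mainly supplying visibility math and small actor, math and AI-sense helpers.
; DT_ObjectVisibility rows turn illumination into normalized visibility, and visibility into clamped detection angle and range.
; Total visibility averages point values with a 0.8 exponent curve.
; Other helpers pick the nearer or farther actor, measure look-at angle, round, inverse-lerp and match senses, where Hear maps to AISense_Damage.
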(fn CalcTotalVisibility
  (params (points :type Array%20of%20BP%20Shadow%20Point%20Comp%20Object%20References))
  (for _array_element points
    (LocalVariables|Setvisibility_sum (+ (LocalVariables|Getvisibility_sum) (Variables|/Game/Blueprints/LightDetection/BP_Shadow_Point_Comp.BP_Shadow_Point_Comp_C|GetVisibility_Value _array_element))))
  (return (Math|Float|Clamp(Float) (Math|Float|Power (/ (LocalVariables|Getvisibility_sum) (Utilities|Array|Length points)) 0.8))))

(fn CalcVisibilityUsingDataTable
  (params (illumination :type Float%20%28double-precision%29) (RowName :type Name :default "Default_Human"))
  (LocalVariables|Setinput_illumination illumination)
  (bind _returnvalue (Utilities|GetDataTableRow "/Game/Blueprints/Data/DT_ObjectVisibility.DT_ObjectVisibility" RowName)
    (:then
      (return (Math|Float|Clamp(Float) (/ (- (LocalVariables|Getinput_illumination) (.illumination_at_zero_visibility (Utilities|Struct|BreakS_Visibility _returnvalue))) (- (.illumination_at_full_visibility (Utilities|Struct|BreakS_Visibility _returnvalue)) (.illumination_at_zero_visibility (Utilities|Struct|BreakS_Visibility _returnvalue)))))))
    (:RowNotFound
      (return 0.0))))

(fn CalcAngleVisibilityUsingDataTable
  (params (RowName :type Name :default "Default_Human") (Visibility :type Float%20%28double-precision%29))
  (bind _returnvalue (Utilities|GetDataTableRow "/Game/Blueprints/Data/DT_ObjectVisibility.DT_ObjectVisibility" RowName)
    (:then
      (return (Math|Float|Clamp(Float) (* (.max_visibility_angle (Utilities|Struct|BreakS_Visibility _returnvalue)) (* Visibility 1.0)) (.min_visibility_angle (Utilities|Struct|BreakS_Visibility _returnvalue)) (.max_visibility_angle (Utilities|Struct|BreakS_Visibility _returnvalue)))))
    (:RowNotFound
      (return 0.0))))

(fn CalcDistanceVisibilityUsingDataTable
  (params (RowName :type Name :default "Default_Human") (Visibility :type Float%20%28double-precision%29))
  (bind _returnvalue (Utilities|GetDataTableRow "/Game/Blueprints/Data/DT_ObjectVisibility.DT_ObjectVisibility" RowName)
    (:then
      (return (Math|Float|Clamp(Float) (* (.max_visibility_range (Utilities|Struct|BreakS_Visibility _returnvalue)) Visibility) (.min_visibility_range (Utilities|Struct|BreakS_Visibility _returnvalue)) (.max_visibility_range (Utilities|Struct|BreakS_Visibility _returnvalue)))))
    (:RowNotFound
      (return 0.0))))

(fn PickActorbyDistance
  (params (pick_most_nearest :type Boolean) (target_a :type Actor%20Object%20Reference) (target_b :type Actor%20Object%20Reference) (start_actor :type Actor%20Object%20Reference))
  (bind _returnvalue (Transformation|GetActorLocation target_a))
  (bind _returnvalue_2 (Transformation|GetActorLocation target_b))
  (bind _returnvalue_3 (Transformation|GetActorLocation start_actor))
  (bind _returnvalue_4 (Math|Vector|Distance(Vector) _returnvalue_3 _returnvalue))
  (bind _returnvalue_5 (Math|Vector|Distance(Vector) _returnvalue_3 _returnvalue_2))
  (bind _returnvalue_6 (< _returnvalue_4 _returnvalue_5))
  (bind _returnvalue_7 (> _returnvalue_4 _returnvalue_5))
  (if pick_most_nearest
    (return (select _returnvalue_6 target_a target_b) (Math|Float|SelectFloat _returnvalue_4 _returnvalue_5 _returnvalue_6))
    (else
      (return (select _returnvalue_7 target_a target_b) (Math|Float|SelectFloat _returnvalue_4 _returnvalue_5 _returnvalue_7)))))

(fn AFindLookatDegrees
  (params (start :type Actor%20Object%20Reference) (target :type Actor%20Object%20Reference))
  (return (Class|KismetMathLibrary|DegAcos (Math|Vector|DotProduct (Transformation|GetActorForwardVector start) (Math|Vector|GetForwardVector (Math|Rotator|FindLookatRotation (Transformation|GetActorLocation start) (Transformation|GetActorLocation target)))))))

(fn RemoveDecimalPart
  (params (value :type Float%20%28double-precision%29) (decimal :type Integer))
  (return (/ (Math|Float|Round (* value decimal)) (Math|Conversions|ToFloat(Integer) decimal))))

(fn InverseLerp
  (params (current_value :type Float%20%28double-precision%29) (min :type Float%20%28double-precision%29) (max :type Float%20%28double-precision%29))
  (return (Math|Float|Clamp(Float) (/ (- current_value min) (- max min)))))

(fn IsSenseClassEqualESense
  (params (sense :type AI%20Sense%20Class%20Reference) (E_Sense :type E_Sense%20Enum :default "NewEnumerator3"))
  (return (== sense (Utilities|Select :Index E_Sense :NewEnumerator3 0 :NewEnumerator0 "/Script/AIModule.AISense_Sight" :NewEnumerator2 "/Script/AIModule.AISense_Damage" :NewEnumerator1 "/Script/AIModule.AISense_Damage"))))