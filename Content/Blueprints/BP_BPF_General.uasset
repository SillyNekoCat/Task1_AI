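; General Blueprint function library of helpers for illumination-based visibility, AI senses, targeting and math.
; Visibility functions read DT_ObjectVisibility rows to normalize illumination to 0–1 and scale view angle and range from a visibility value within row limits.
; TeamCheck compares actors' gameplay tags, while other helpers pick actors by distance or tag, measure look-at angles, round and inverse-lerp.
; The sense-class comparison maps both Hear and Damage to AISense_Damage.
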(fn CalcVisibilityUsingDataTable
  (params (illumination :type Float%20%28double-precision%29) (RowName :type Name :default "Default_Human"))
  (LocalVariables|Setinput_illumination illumination)
  (bind _returnvalue (Utilities|GetDataTableRow "/Game/Blueprints/Data/DT_ObjectVisibility.DT_ObjectVisibility" RowName)
    (:then
      (return (Math|Float|Clamp(Float) (/ (- (LocalVariables|Getinput_illumination) (.illumination_at_zero_visibility (Utilities|Struct|BreakS_Visibility _returnvalue))) (- (.illumination_at_full_visibility (Utilities|Struct|BreakS_Visibility _returnvalue)) (.illumination_at_zero_visibility (Utilities|Struct|BreakS_Visibility _returnvalue)))))))
    (:RowNotFound
      (return 0.0))))

(fn CalcAngleVisibilityUsingDataTable
  (params (RowName :type Name :default "Default_Human") (Visibility :type Float%20%28double-precision%29))
  (bind _returnvalue (Utilities|GetDataTableRow "/Game/Blueprints/Data/DT_ObjectVisibility.DT_ObjectVisibility" RowName)
    (:then
      (return (Math|Float|Clamp(Float) (* (.max_visibility_angle (Utilities|Struct|BreakS_Visibility _returnvalue)) (* Visibility 1.0)) (.min_visibility_angle (Utilities|Struct|BreakS_Visibility _returnvalue)) (.max_visibility_angle (Utilities|Struct|BreakS_Visibility _returnvalue)))))
    (:RowNotFound
      (return 0.0))))

(fn CalcDistanceVisibilityUsingDataTable
  (params (RowName :type Name :default "Default_Human") (Visibility :type Float%20%28double-precision%29))
  (bind _returnvalue (Utilities|GetDataTableRow "/Game/Blueprints/Data/DT_ObjectVisibility.DT_ObjectVisibility" RowName)
    (:then
      (return (Math|Float|Clamp(Float) (* (.max_visibility_range (Utilities|Struct|BreakS_Visibility _returnvalue)) Visibility) (.min_visibility_range (Utilities|Struct|BreakS_Visibility _returnvalue)) (.max_visibility_range (Utilities|Struct|BreakS_Visibility _returnvalue)))))
    (:RowNotFound
      (return 0.0))))

(fn PickActorbyDistance
  (params (pick_most_nearest :type Boolean) (target_a :type Actor%20Object%20Reference) (target_b :type Actor%20Object%20Reference) (start_actor :type Actor%20Object%20Reference))
  (bind _returnvalue (Transformation|GetActorLocation target_a))
  (bind _returnvalue_2 (Transformation|GetActorLocation target_b))
  (bind _returnvalue_3 (Transformation|GetActorLocation start_actor))
  (bind _returnvalue_4 (Math|Vector|Distance(Vector) _returnvalue_3 _returnvalue))
  (bind _returnvalue_5 (Math|Vector|Distance(Vector) _returnvalue_3 _returnvalue_2))
  (bind _returnvalue_6 (< _returnvalue_4 _returnvalue_5))
  (bind _returnvalue_7 (> _returnvalue_4 _returnvalue_5))
  (if pick_most_nearest
    (return (select _returnvalue_6 target_a target_b) (Math|Float|SelectFloat _returnvalue_4 _returnvalue_5 _returnvalue_6))
    (else
      (return (select _returnvalue_7 target_a target_b) (Math|Float|SelectFloat _returnvalue_4 _returnvalue_5 _returnvalue_7)))))

(fn FindLookatDegrees
  (params (start_fwd_vector :type Vector) (start_loc :type Vector) (target_loc :type Vector%20%28by%20ref%29))
  (return (Class|KismetMathLibrary|DegAcos (Math|Vector|DotProduct start_fwd_vector (Math|Vector|GetForwardVector (Math|Rotator|FindLookatRotation start_loc target_loc))))))

(fn RemoveDecimalPart
  (params (value :type Float%20%28double-precision%29) (decimal :type Integer))
  (return (/ (Math|Float|Round (* value decimal)) (Math|Conversions|ToFloat(Integer) decimal))))

(fn InverseLerp
  (params (current_value :type Float%20%28double-precision%29) (min :type Float%20%28double-precision%29) (max :type Float%20%28double-precision%29))
  (return (Math|Float|Clamp(Float) (/ (- current_value min) (- max min)))))

(fn IsSenseClassEqualESense
  (params (sense :type AI%20Sense%20Class%20Reference) (E_Sense :type E_Sense%20Enum :default "NewEnumerator3"))
  (return (== sense (Utilities|Select :Index E_Sense :NewEnumerator3 0 :NewEnumerator0 "/Script/AIModule.AISense_Sight" :NewEnumerator2 "/Script/AIModule.AISense_Damage" :NewEnumerator1 "/Script/AIModule.AISense_Damage"))))

(fn TeamCheck
  (params (actor_1 :type Actor%20Object%20Reference) (actor_2 :type Actor%20Object%20Reference))
  (if (and (Utilities|DoesObjectImplementInterface actor_1 "/Script/GameplayTags.GameplayTagAssetInterface") (Utilities|DoesObjectImplementInterface actor_2 "/Script/GameplayTags.GameplayTagAssetInterface"))
    (bind _tagcontainer (GameplayTags|GetOwnedGameplayTags actor_1 :!class /Script/GameplayTags.GameplayTagAssetInterface))
    (bind _tagcontainer_2 (GameplayTags|GetOwnedGameplayTags actor_2 :!class /Script/GameplayTags.GameplayTagAssetInterface))
    (if (or (GameplayTags|HasTag _tagcontainer "(TagName=\"Team.NotValid\")") (GameplayTags|HasTag _tagcontainer_2 "(TagName=\"Team.NotValid\")"))
      (return "NewEnumerator0")
      (else
        (return (select (GameplayTags|HasAnyTags _tagcontainer_2 _tagcontainer) "NewEnumerator1" "NewEnumerator2"))))
    (else
      (return "NewEnumerator0"))))

(fn NearestActorwithTag
  (params (input_actors :type Array%20of%20Actor%20Object%20References) (input_tag :type Name :default "Interact") (input_target :type Actor%20Object%20Reference))
  (if (Utilities|Array|IsNotEmpty input_actors)
    (for _array_element input_actors
      (if (Actor|ActorHasTag _array_element input_tag)
        (Utilities|FlowControl|Sequence
          (:then_0
            (Utilities|FlowControl|DoOnce false
              (:Completed
                (LocalVariables|Setlowest_dist (Transformation|GetDistanceTo _array_element input_target)))))
          (:then_1
            (if (>= (LocalVariables|Getlowest_dist) (Transformation|GetDistanceTo _array_element input_target))
              (LocalVariables|Setlowest_dist (Transformation|GetDistanceTo _array_element input_target))
              (LocalVariables|Setresult_actor _array_element))))))
    (return (LocalVariables|Getresult_actor))))