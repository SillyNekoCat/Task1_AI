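; BP_Button is a pressure button that activates its target actors while a tagged component rests on it.
; Box overlaps with InteractTag components play a Timeline that moves Cube1 along Z from its construction-time height, reversing once no tagged component remains.
; When the Timeline finishes, each valid entry in InteractTargets receives an activation message: true when pressed, false when released.
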(event OnComponentBeginOverlap(Box)
  (params (OverlappedComponent :type Primitive%20Component%20Object%20Reference) (OtherActor :type Actor%20Object%20Reference) (OtherComp :type Primitive%20Component%20Object%20Reference) (OtherBodyIndex :type Integer) (bFromSweep :type Boolean) (SweepResult :type Hit%20Result%20Structure%20%28by%20ref%29))
  (if (not (Variables|Default|Getoverlap_interact))
    (if (Components|ComponentHasTag OtherComp (Variables|Default|GetInteract_Tag))
      (Variables|Default|Setoverlap_interact true)
      (bind (_direction _pos) (Timeline|Timeline Play)
        (:Update
          (Transformation|SetRelativeLocation (Variables|Default|GetCube1) (Math|Vector|MakeVectorNetQuantize 0.0 0.0 (Math|Float|Lerp 1.0 (Variables|Default|GetDefault_z) _pos)) false false))
        (:Finished
          (for _array_element (Variables|Default|GetInteract_Targets)
            (Utilities|IsValid _array_element
              (:Is%20Valid
                (Class|BPIInteract|SetActivation(Message) _array_element (Utilities|Select :Index _direction :Forward true :Backward false))))))))))

(event OnComponentEndOverlap(Box)
  (params (OverlappedComponent :type Primitive%20Component%20Object%20Reference) (OtherActor :type Actor%20Object%20Reference) (OtherComp :type Primitive%20Component%20Object%20Reference) (OtherBodyIndex :type Integer))
  (bind _components_with_tag (CallFunction|GetOverlappingComponentswithTag (Variables|Default|GetBox) (Variables|Default|GetInteract_Tag)))
  (if (Utilities|Array|IsEmpty _components_with_tag)
    (Variables|Default|Setoverlap_interact false)
    (bind (_direction _pos) (Timeline|Timeline Reverse)
      (:Update
        (Transformation|SetRelativeLocation (Variables|Default|GetCube1) (Math|Vector|MakeVectorNetQuantize 0.0 0.0 (Math|Float|Lerp 1.0 (Variables|Default|GetDefault_z) _pos)) false false))
      (:Finished
        (for _array_element (Variables|Default|GetInteract_Targets)
          (Utilities|IsValid _array_element
            (:Is%20Valid
              (Class|BPIInteract|SetActivation(Message) _array_element (Utilities|Select :Index _direction :Forward true :Backward false)))))))))

(event EventBeginPlay)

(event Collision|EventActorBeginOverlap
  (params (OtherActor :type Actor%20Object%20Reference)))

(event EventTick
  (params (DeltaSeconds :type Float%20%28single-precision%29)))

(fn ConstructionScript
  (Variables|Default|SetDefault_z (.Z (Math|Vector|BreakVector (Variables|/Script/Engine.SceneComponent|GetRelativeLocation (Variables|Default|GetCube1))))))

(fn GetOverlappingComponentswithTag
  (params (Target :type Primitive%20Component%20Object%20Reference) (Tag :type Name))
  (for _array_element (Class|PrimitiveComponent|GetOverlappingComponents Target)
    (if (Components|ComponentHasTag _array_element Tag)
      (Utilities|Array|AddUnique (LocalVariables|Getresult_components_with_tag) _array_element)))
  (return (LocalVariables|Getresult_components_with_tag)))