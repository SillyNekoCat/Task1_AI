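; BP_InputButton is an interactable button that animates a cube and passes activation on to linked targets.
; Activation plays a timeline that lerps Cube1's relative Z between a fixed height and the height cached in the construction script.
; When the timeline finishes, each valid InteractTargets entry receives an activation message based on timeline direction.
; Only activation is handled; a deactivation call does nothing, so the timeline is never reversed.
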(event Custom|Event_SetActivation
  (params (is_active :type Boolean))
  (if is_active
    (bind (_direction _pos) (Timeline|Timeline Play)
      (:Update
        (Transformation|SetRelativeLocation (Variables|Default|GetCube1) (Math|Vector|MakeVectorNetQuantize 0.0 0.0 (Math|Float|Lerp 1.2e+02 (Variables|Default|GetDefault_z) _pos)) false false))
      (:Finished
        (for _array_element (Variables|Default|GetInteract_Targets)
          (Utilities|IsValid _array_element
            (:Is%20Valid
              (Class|BPIInteract|SetActivation(Message) _array_element (Utilities|Select :Index _direction :Forward true :Backward false)))))))))

(event EventBeginPlay)

(event Collision|EventActorBeginOverlap
  (params (OtherActor :type Actor%20Object%20Reference)))

(event EventTick
  (params (DeltaSeconds :type Float%20%28single-precision%29)))

(fn ConstructionScript
  (Variables|Default|SetDefault_z (.Z (Math|Vector|BreakVector (Variables|/Script/Engine.SceneComponent|GetRelativeLocation (Variables|Default|GetCube1))))))

(fn SetActivation
  (params (is_active :type Boolean))
  (CallFunction|EventSetActivation is_active)
  (return true))