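; Combat component that handles equipping, hiding and attacking with a weapon for its owning character, with AI controller hooks.
; It spawns the weapon hidden, attaches it to the owner's skeletal mesh, and toggles visibility on montage notifies or immediately without animation.
; Attacks play a random weapon montage behind an IsAttacking guard, notifying the owner and firing result dispatchers.
; Strafe and attack radius setters forward values to the AI controller through interface messages.
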(event Custom|Attack
  (params (clear_focus_OnBlendOut :type Boolean))
  (bind _returnvalue (Components|GetOwner))
  (bind _current_weapon (Variables|Default|GetCurrent_Weapon))
  ;[1 1 1] Attack
  (if (Variables|Default|GetIs_Holding_Weapon)
    (Utilities|IsValid _current_weapon
      (:Is%20Valid
        (bind _montages (Class|BPIWeapon|GetWeaponMontages(Message) _current_weapon))
        (if (Utilities|Array|IsEmpty _montages)
          (Default|CallOnAttackEnd false :!label _label)
          (elif (Variables|Default|GetIs_Attacking)
            (goto _label)
            (else
              (Variables|Default|SetIs_Attacking true)
              (Utilities|IsValid (.OutItem (Utilities|Array|Random _montages))
                (:Is%20Valid
                  (Class|BPIMovementControl|AttackBegin(Message) (Components|GetOwner))
                  (Animation|Montage|PlayMontage (Variables|Default|GetOwner_SkeletalMesh) (.OutItem (Utilities|Array|Random _montages))
                    (:OnCompleted
                      (Variables|Default|SetIs_Attacking false)
                      (Class|BPIMovementControl|AttackEnd(Message) _returnvalue)
                      (Default|CallOnAttackEnd true))
                    (:OnBlendOut
                      (if clear_focus_OnBlendOut
                        (AI|ClearFocus (AI|GetAIController (Components|GetOwner)))))
                    (:OnInterrupted
                      (Variables|Default|SetIs_Attacking false)
                      (Class|BPIMovementControl|AttackEnd(Message) _returnvalue)
                      (Default|CallOnAttackEnd false))))
                (:Is%20Not%20Valid
                  (Default|CallOnAttackEnd false)))))))
      (:Is%20Not%20Valid
        (Default|CallOnAttackEnd false :!label _label_2)))
    (else
      (goto _label_2))))

(event Custom|Equip_Weapon
  (params (no_anim :type Boolean))
  ;[1 1 1] Equip Weapon
  (if (not (Variables|Default|GetIs_Holding_Weapon))
    (if (Variables|Default|GetIs_WeaponAttached)
      _
      (else
        (CallFunction|CreateAttachWeaponinHand)))
    (if no_anim
      (CallFunction|InitWeapon true :!label _label)
      (Default|CallOnEquipWeapon (Variables|Default|GetIs_Holding_Weapon))
      (else
        (bind _montage (Class|BPIWeapon|GetEquipMontage(Message) (Variables|Default|GetCurrent_Weapon)))
        (Utilities|IsValid _montage
          (:Is%20Valid
            (bind _notifyname (Animation|Montage|PlayMontage (Variables|Default|GetOwner_SkeletalMesh) _montage)
              (:OnCompleted
                (Default|CallOnEquipWeapon (Variables|Default|GetIs_Holding_Weapon) :!label _label_2))
              (:OnInterrupted
                (goto _label_2))
              (:OnNotifyBegin
                (switch name _notifyname
                  (:Equip
                    (CallFunction|InitWeapon true))))))
          (:Is%20Not%20Valid
            (goto _label)))))
    (else
      (Default|CallOnEquipWeapon (Variables|Default|GetIs_Holding_Weapon)))))

(event Custom|Hide_Weapon
  (params (no_anim :type Boolean))
  ;[1 1 1] Hide Weapon
  (if (Variables|Default|GetIs_Holding_Weapon)
    (if no_anim
      (CallFunction|InitWeapon false :!label _label)
      (Default|CallOnHideWeapon (not (Variables|Default|GetIs_Holding_Weapon)))
      (else
        (bind _montage (Class|BPIWeapon|GetHideMontage(Message) (Variables|Default|GetCurrent_Weapon)))
        (Utilities|IsValid _montage
          (:Is%20Valid
            (bind _notifyname (Animation|Montage|PlayMontage (Variables|Default|GetOwner_SkeletalMesh) _montage)
              (:OnCompleted
                (Default|CallOnHideWeapon (not (Variables|Default|GetIs_Holding_Weapon)) :!label _label_2))
              (:OnInterrupted
                (goto _label_2))
              (:OnNotifyBegin
                (switch name _notifyname
                  (:Hide
                    (CallFunction|InitWeapon false))))))
          (:Is%20Not%20Valid
            (goto _label)))))
    (else
      (Default|CallOnHideWeapon (not (Variables|Default|GetIs_Holding_Weapon))))))

(event EventBeginPlay
  (Variables|Default|SetOwner_SkeletalMesh (Actor|GetComponentbyClass (Components|GetOwner) "/Script/Engine.SkeletalMeshComponent"))
  (if (Variables|Default|GetHolding_Weapon_FromBeginPlay)
    (CallFunction|EquipWeapon true)))

(event EventTick
  (params (DeltaSeconds :type Float%20%28single-precision%29)))

(fn CreateAttachWeaponinHand
  (bind _weapon_class (Variables|Default|GetWeapon_Class))
  (if (Utilities|IsValidClass _weapon_class)
    (bind _returnvalue (Game|SpawnActorfromClass _weapon_class (Transformation|GetActorTransform (Components|GetOwner)) "Undefined" "MultiplyWithRoot" 0 0))
    (bind _output_get (Variables|Default|SetCurrent_Weapon _returnvalue))
    (Rendering|SetActorHiddenInGame _output_get true)
    (CallFunction|AttachWeapon _output_get)))

(fn DestroyWeaponinHand
  (bind _current_weapon (Variables|Default|GetCurrent_Weapon))
  (Utilities|IsValid _current_weapon
    (:Is%20Valid
      (Actor|DestroyActor _current_weapon)
      (CallFunction|SetIsHoldingWeapon false))))

(fn SetStrafeRadius
  (params (input_strafe_radius :type Float%20%28double-precision%29))
  (bind _output_get (Variables|Default|SetStrafe_Radius input_strafe_radius))
  (Class|BPIAI|SetStrafeRadius(Message) (AI|GetAIController (Components|GetOwner)) _output_get))

(fn GetStrafeRadius
  (return (Variables|Default|GetStrafe_Radius)))

(fn SetAttackRadius
  (params (input_strafe_radius :type Float%20%28double-precision%29))
  (bind _output_get (Variables|Default|SetAttack_Radius input_strafe_radius))
  (Class|BPIAI|SetAttackRadius(Message) (AI|GetAIController (Components|GetOwner)) _output_get))

(fn GetAttackRadius
  (return (Variables|Default|GetAttack_Radius)))

(fn SetIsHoldingWeapon
  (params (input :type Boolean))
  (bind _output_get (Variables|Default|SetIs_Holding_Weapon input))
  (Default|CallOnIsHoldingWeaponChange _output_get))

(fn AttachWeapon
  (params (weapon :type Actor%20Object%20Reference))
  (bind _success (Class|BPIWeapon|AttachWeapon(Message) weapon (Variables|Default|GetOwner_SkeletalMesh)))
  (if _success
    (Class|BPIWeapon|SetWeaponOwner(Message) (Variables|Default|GetCurrent_Weapon) (Components|GetOwner))
    (Variables|Default|SetIs_WeaponAttached true)))

(fn InitWeapon
  (params (init :type Boolean))
  (if init
    (Rendering|SetActorHiddenInGame (Variables|Default|GetCurrent_Weapon) false)
    (CallFunction|SetIsHoldingWeapon true)
    (else
      (Rendering|SetActorHiddenInGame (Variables|Default|GetCurrent_Weapon) true)
      (CallFunction|SetIsHoldingWeapon false))))