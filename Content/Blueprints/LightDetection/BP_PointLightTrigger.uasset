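; BP_PointLightTrigger is a light-detection actor that pairs a point light with a sphere whose radius matches the light's reach.
; The construction script applies exposed intensity, attenuation radius and color to the light, then sizes the sphere to that attenuation radius.
; Getter functions expose the light component, intensity, radius and falloff exponent.
; The game-mode debug change event calls its parent, then toggles the sphere's debug visibility.
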(event EventBeginPlay
  (|CallParentFunction) ; This node is disabled and will not be called.\nDrag off pins to build functionality.
)

(event Collision|EventActorBeginOverlap
  (params (OtherActor :type Actor%20Object%20Reference))
  (|CallParentFunction OtherActor) ; This node is disabled and will not be called.\nDrag off pins to build functionality.
)

(event EventTick
  (params (DeltaSeconds :type Float%20%28single-precision%29))
  (|CallParentFunction DeltaSeconds) ; This node is disabled and will not be called.\nDrag off pins to build functionality.
)

(event EventOnGMDebugChangeEvent
  (params (debug :type Boolean))
  (|CallParentFunction debug)
  (CallFunction|SetVisibilityDebug (Variables|Default|GetSphere) debug))

(fn ConstructionScript
  (|CallParentFunction)
  (Utilities|FlowControl|Sequence
    (:then_0
      (Rendering|Components|Light|SetIntensity (Variables|Default|GetPointLight) (Variables|Default|GetIntensity_param))
      (Rendering|Lighting|SetAttenuationRadius (Variables|Default|GetPointLight) (Variables|Default|GetAttenationRadius_param))
      (Rendering|Components|Light|SetLightColor (Variables|Default|GetPointLight) (Variables|Default|GetLight_Color_param) true))
    (:then_1
      (Components|Sphere|SetSphereRadius (Variables|Default|GetSphere) (Variables|/Script/Engine.LocalLightComponent|GetAttenuationRadius (Variables|Default|GetPointLight)) true))))

(fn GetAttenuationRadius
  (return (Variables|/Script/Engine.LocalLightComponent|GetAttenuationRadius (Variables|Default|GetPointLight))))

(fn GetIntensity
  (return (Variables|/Script/Engine.LightComponentBase|GetIntensity (Variables|Default|GetPointLight))))

(fn GetLightFalloffExponent
  (params (optional_target_loc :type Vector :default "0, 0, 0"))
  (return (Variables|/Script/Engine.PointLightComponent|GetLightFalloffExponent (Variables|Default|GetPointLight))))

(fn GetLightComp
  (return (Variables|Default|GetPointLight)))