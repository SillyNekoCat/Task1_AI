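; Actor component that measures how lit or shadowed its owner is, broadcasting total visibility and its inverse shadow value.
; Each owner-supplied point takes the strongest overlapping light trigger passing cone and line-trace checks, converting falloff-based illumination to visibility via data table.
; Point values are averaged, power-curved and clamped.
; Overlaps and observer increments trigger rechecks, and Tick runs only while points overlap lights or observers exist, with game-mode-toggled debug drawing.
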(event Custom|On_GM_DebugChange_Event
  (params (debug :type Boolean))
  ;[1 0.886 0] debug
  (bind _output_get (Variables|Default|SetDebug debug))
  (bind _keys (Utilities|Map|Keys (Variables|Default|GetPointsAndVisibility)))
  (for _array_element _keys
    (Development|SetHiddeninGame _array_element (not _output_get) false)))

(event Custom|BeginOverlap
  (params (OverlappedComponent :type Primitive%20Component%20Object%20Reference) (OtherActor :type Actor%20Object%20Reference) (OtherComp :type Primitive%20Component%20Object%20Reference) (OtherBodyIndex :type Integer) (bFromSweep :type Boolean) (SweepResult :type Hit%20Result%20Structure%20%28by%20ref%29))
  ;[1 1 1] Init
  (CallFunction|OnPointBeginEndOverlap OtherActor))

(event Custom|EndOverlap
  (params (OverlappedComponent :type Primitive%20Component%20Object%20Reference) (OtherActor :type Actor%20Object%20Reference) (OtherComp :type Primitive%20Component%20Object%20Reference) (OtherBodyIndex :type Integer))
  ;[1 1 1] Init
  (CallFunction|OnPointBeginEndOverlap OtherActor))

(event EventBeginPlay
  (Utilities|FlowControl|Sequence
    (:then_0
      ;[1 1 1] Init
      (bind _components (Class|BPIVisibility|GetShadowPoints(Message) (Components|GetOwner)))
      (for _array_element _components
        (Utilities|Map|Add (Variables|Default|GetPointsAndVisibility) _array_element 0.0)
        (Collision|AssignOnComponentBeginOverlap _array_element (delegate Custom|BeginOverlap))
        (Collision|BindEventtoOnComponentEndOverlap _array_element (delegate Custom|EndOverlap)))
      (CallFunction|PointsCheck))
    (:then_1
      ;[1 0.886 0] debug
      (bind _asbp_gm_base_debug (Utilities|Casting|CastToBP_GM_BaseDebug (Game|GetGameMode)))
      (EventDispatchers|AssignOnGMDebugChange _asbp_gm_base_debug (delegate Custom|On_GM_DebugChange_Event)))))

(event EventTick
  (params (DeltaSeconds :type Float%20%28single-precision%29))
  (CallFunction|PointsCheck))

(fn GetShadowValue
  (return (Variables|Default|GetShadow_Value)))

(fn SetTotalVisibility
  (params (TotalVisibility :type Float%20%28double-precision%29))
  (Variables|Default|SetTotalVisibility (Math|Float|Clamp(Float) TotalVisibility (- 1.0 (Variables|Default|GetMax_Shadow_Value))))
  (Variables|Default|SetShadow_Value (- 1.0 (Variables|Default|GetTotalVisibility)))
  (Default|CallOnTotalVisibilityChange (Components|GetOwner) self (Variables|Default|GetTotalVisibility) (Variables|Default|GetShadow_Value)))

(fn GetTotalVisibility
  (return (Variables|Default|GetTotalVisibility)))

(fn GetOverlapPoints
  (bind _components (Class|BPIVisibility|GetShadowPoints(Message) (Components|GetOwner)))
  (for _array_element _components
    (if (CallFunction|IsPointOverlap _array_element)
      (Utilities|Array|AddUnique (LocalVariables|Getlocal_points) _array_element)))
  (return (LocalVariables|Getlocal_points)))

(fn PointsCheck
  (Utilities|FlowControl|Sequence
    (:then_0
      (bind _keys (Utilities|Map|Keys (Variables|Default|GetPointsAndVisibility)))
      (for _array_element _keys
        (Utilities|FlowControl|Sequence
          (:then_0
            ;[1 1 1] Calc visibility for every point
            (if (CallFunction|IsPointOverlap _array_element)
              (LocalVariables|Setis_any_point_overlap_light true)
              (CallFunction|SinglePointCheck (Variables|Default|GetObjVisibility_RowName) _array_element)
              (else
                (CallFunction|SetPointVisibility _array_element 0.0))))
          (:then_1
            ;[1 1 1] Visibility sum
            (LocalVariables|Setvisibility_sum (+ (LocalVariables|Getvisibility_sum) (.Value (Utilities|Map|Find (Variables|Default|GetPointsAndVisibility) _array_element)))))))
      ;[1 1 1] Calc avarage visibility, Enable/Disable Tick
      (if (LocalVariables|Getis_any_point_overlap_light)
        (CallFunction|SetTotalVisibility (Math|Float|Power (/ (LocalVariables|Getvisibility_sum) (Utilities|Array|Length _keys)) 0.8))
        (if (not (Class|ActorComponent|IsComponentTickEnabled)) :!label _label
          (Components|Tick|SetComponentTickEnabled true))
        (else
          (CallFunction|SetTotalVisibility 0.0)
          (if (> (Variables|Default|GetObservers) 0)
            (goto _label)
            (elif (Class|ActorComponent|IsComponentTickEnabled)
              (Components|Tick|SetComponentTickEnabled false))))))
    (:then_1
      ;[1 0.8759 0] Debug
      (if (Variables|Default|GetDebug)
        (CallFunction|Debug1)))))

(fn IncrementObservers
  (Math|Integer|IncrementInt (Variables|Default|GetObservers)
    (:%20%20
      (CallFunction|PointsCheck))))

(fn DecrementObservers
  (Math|Integer|DecrementInt (Variables|Default|GetObservers)))

(fn Debug1
  (bind _returnvalue (Components|GetOwner))
  (bind _returnvalue_2 (Math|Float|MakeLiteralFloat 0.0))
  (bind _returnvalue_3 (Transformation|GetActorLocation _returnvalue))
  (bind _returnvalue_4 (+ _returnvalue_3 "0.000000,0.000000,130.000000"))
  (bind _returnvalue_5 (+ _returnvalue_4 "0.000000,0.000000,10.000000"))
  (bind _returnvalue_6 (+ _returnvalue_5 "0.000000,0.000000,10.000000"))
  (Rendering|Debug|DrawDebugString _returnvalue_4 (Utilities|String|Append "Observers:   " (Utilities|String|ToString(Integer) (Variables|Default|GetObservers))) 0 "(R=0.079221,G=0.760525,B=0.481000,A=1.000000)" _returnvalue_2)
  (Rendering|Debug|DrawDebugString _returnvalue_5 (Utilities|String|Append "TOTAL VISIBILITY:  " (Utilities|String|ToString(Float) (Variables|Default|GetTotalVisibility))) 0 "(R=1.000000,G=1.000000,B=1.000000,A=1.000000)" _returnvalue_2)
  (bind _angle (CallFunction|CalcAngleVisibilityUsingDataTable (Variables|Default|GetObjVisibility_RowName) (Variables|Default|GetTotalVisibility)))
  (Rendering|Debug|DrawDebugString _returnvalue_6 (Utilities|String|Append "VISIBILITY ANGLE:  " (Utilities|String|ToString(Float) _angle)) 0 "(R=1.000000,G=0.182158,B=0.000000,A=1.000000)" _returnvalue_2)
  (bind _distance (CallFunction|CalcDistanceVisibilityUsingDataTable (Variables|Default|GetObjVisibility_RowName) (Variables|Default|GetTotalVisibility)))
  (Rendering|Debug|DrawDebugString (+ _returnvalue_6 "0.000000,0.000000,10.000000") (Utilities|String|Append "VISIBILITY DISTANCE:   " (Utilities|String|ToString(Float) _distance)) 0 "(R=1.000000,G=0.898375,B=0.565361,A=1.000000)" _returnvalue_2))

(fn GetPointOverlappingActors
  (params (input_prim_comp :type Primitive%20Component%20Object%20Reference))
  (return (Collision|GetOverlappingActors input_prim_comp "/Game/Blueprints/LightDetection/BP_BaseLightTrigger.BP_BaseLightTrigger_C" :!class /Script/Engine.PrimitiveComponent)))

(fn IsPointOverlap
  (params (input_prim_comp :type Primitive%20Component%20Object%20Reference))
  (return (Utilities|Array|IsNotEmpty (CallFunction|GetPointOverlappingActors input_prim_comp))))

(fn CalcIlluminationValue
  (params (input_distance :type Float%20%28double-precision%29) (input_light :type Object%20Object%20Reference) (input_point :type Primitive%20Component%20Object%20Reference))
  (bind _radius (Class|BPILightTrigger|GetAttenuationRadius(Message) input_light))
  (LocalVariables|Setinput_radius _radius)
  (if (> input_distance (LocalVariables|Getinput_radius))
    (return 0.0)
    (else
      (bind _intensity (Class|BPILightTrigger|GetIntensity(Message) input_light))
      (LocalVariables|Setinput_intensity _intensity)
      (bind _value (Class|BPILightTrigger|GetLightFalloffExponent(Message) input_light (Transformation|GetWorldLocation input_point)))
      (LocalVariables|Setinput_falloff_exponent _value)
      (return (Utilities|IlluminationFormula input_distance (LocalVariables|Getinput_radius) (/ (LocalVariables|Getinput_falloff_exponent) 1.15))))))

(fn SinglePointCheck
  (params (RowName :type Name) (input_point :type Primitive%20Component%20Object%20Reference))
  (bind _returnvalue (Transformation|GetWorldLocation input_point))
  (bind _returnvalue_2 (+ _returnvalue "0.000000,0.000000,-6.000000"))
  (Utilities|FlowControl|Sequence
    (:then_0
      (LocalVariables|Setpoint_loc (Transformation|GetWorldLocation input_point))
      (for _array_element (CallFunction|GetPointOverlappingActors input_point)
        (Utilities|FlowControl|Sequence ; find light source that gives highest illumination
          (:then_0
            (bind _output_get (LocalVariables|Setarr_current_light _array_element))
            (LocalVariables|Setarr_current_light_loc (Transformation|GetActorLocation _output_get)))
          (:then_1
            ;[1 1 1] Check light outer angle
            (bind _outer_angle (Class|BPILightTrigger|GetOuterAngle(Message) (LocalVariables|Getarr_current_light)))
            (if (>= _outer_angle 0.0)
              (bind _comp (Class|BPILightTrigger|GetLightComp(Message) (LocalVariables|Getarr_current_light)))
              (Utilities|IsValid _comp
                (:Is%20Valid
                  (if (<= (CallFunction|FindLookatDegrees (Math|Vector|GetForwardVector _comp) (LocalVariables|Getarr_current_light_loc) (LocalVariables|Getpoint_loc)) _outer_angle)
                    ;[1 1 1] is path of light not blocked
                    (bind _outhit (Collision|LineTraceByChannel (LocalVariables|Getarr_current_light_loc) (LocalVariables|Getpoint_loc) "TraceTypeQuery1" false 0 (select (Variables|Default|GetDebug) "ForOneFrame" "None") true "(R=0.145833,G=0.613801,B=1.000000,A=1.000000)" "(R=1.000000,G=0.000000,B=0.000000,A=1.000000)" 0.3 :!label _label))
                    (if (not (.bBlockingHit (Collision|BreakHitResult _outhit)))
                      ;[1 1 1] calc highest illumination
                      (bind _illumination (CallFunction|CalcIlluminationValue (Math|Vector|Distance(Vector) (LocalVariables|Getarr_current_light_loc) (LocalVariables|Getpoint_loc)) (LocalVariables|Getarr_current_light) input_point))
                      (if (> _illumination (LocalVariables|Gethighest_illumination))
                        (LocalVariables|Sethighest_illumination _illumination)
                        (LocalVariables|Setlocal_distance (Math|Vector|Distance(Vector) (LocalVariables|Getarr_current_light_loc) (LocalVariables|Getpoint_loc))))))))
              (else
                (goto _label))))))
      ;[1 1 1] calc highest visibility
      (bind _visibility (CallFunction|CalcVisibilityUsingDataTable (LocalVariables|Gethighest_illumination) RowName))
      (LocalVariables|Setlocal_vis _visibility)
      (CallFunction|SetPointVisibility input_point _visibility))
    (:then_1
      ;[1 0.9144 0] Debug
      (if (Variables|Default|GetDebug)
        (Rendering|Debug|DrawDebugString _returnvalue (Utilities|String|Append "vis: " (Utilities|String|ToString(Float) (CallFunction|RemoveDecimalPart (LocalVariables|Getlocal_vis) 100))) 0 "(R=1.000000,G=1.000000,B=1.000000,A=1.000000)")
        (Rendering|Debug|DrawDebugString _returnvalue_2 (Utilities|String|Append "dist: " (Utilities|String|ToString(Float) (CallFunction|RemoveDecimalPart (LocalVariables|Getlocal_distance) 10))) 0 "(R=0.000000,G=0.729663,B=1.000000,A=1.000000)")
        (Rendering|Debug|DrawDebugString (+ _returnvalue_2 "0.000000,0.000000,-6.000000") (Utilities|String|Append "ill:  " (Utilities|String|ToString(Float) (CallFunction|RemoveDecimalPart (LocalVariables|Gethighest_illumination) 100))) 0 "(R=0.838913,G=0.558058,B=1.000000,A=1.000000)")))))

(fn SetPointVisibility
  (params (input_point :type Primitive%20Component%20Object%20Reference) (input_visibility :type Float%20%28double-precision%29))
  (Utilities|Map|Add (Variables|Default|GetPointsAndVisibility) input_point input_visibility))

(fn OnPointBeginEndOverlap
  (params (input_actor :type Actor%20Object%20Reference))
  (Utilities|IsValid input_actor
    (:Is%20Valid
      (if (Actor|ActorHasTag input_actor "LightTrigger")
        (CallFunction|PointsCheck :!label _label)))
    (:Is%20Not%20Valid
      (goto _label))))