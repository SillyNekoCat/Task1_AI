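; Shadow point component for light detection that calculates how visible its position is under nearby lights.
; It tracks overlapping light triggers, line-traces from each, and keeps the strongest unblocked illumination, based on distance, radius and falloff.
; A data-table lookup converts that to visibility and broadcasts it, resetting to zero outside all triggers.
; Tick recalculates only while NoObserversCalc is set and lights overlap; GameMode debug toggles on-screen readouts.
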(event Custom|On_GM_DebugChange_Event
  (params (debug :type Boolean))
  ;[1 0.886 0] debug
  (bind _output_get (Variables|Default|SetDebug debug))
  (Development|SetHiddeninGame (not _output_get) false))

(event Custom|OnComponentBeginOverlap_Event
  (params (OverlappedComponent :type Primitive%20Component%20Object%20Reference) (OtherActor :type Actor%20Object%20Reference) (OtherComp :type Primitive%20Component%20Object%20Reference) (OtherBodyIndex :type Integer) (bFromSweep :type Boolean) (SweepResult :type Hit%20Result%20Structure%20%28by%20ref%29))
  (if (Actor|ActorHasTag OtherActor "LightTrigger")
    (Utilities|Array|AddUnique (Variables|Default|GetOverlapping_LightTriggers) OtherActor)
    (CallFunction|EnableTickCalc true)))

(event Custom|OnComponentEndOverlap_Event
  (params (OverlappedComponent :type Primitive%20Component%20Object%20Reference) (OtherActor :type Actor%20Object%20Reference) (OtherComp :type Primitive%20Component%20Object%20Reference) (OtherBodyIndex :type Integer))
  (if (Actor|ActorHasTag OtherActor "LightTrigger")
    (Variables|Default|SetOverlapping_LightTriggers (Collision|GetOverlappingActors "/Game/Blueprints/LightDetection/BP_BaseLightTrigger.BP_BaseLightTrigger_C" :!class /Script/Engine.PrimitiveComponent))
    (if (Utilities|Array|IsEmpty (Variables|Default|GetOverlapping_LightTriggers))
      (CallFunction|SetVisibilityValue 0.0)
      (CallFunction|EnableTickCalc false)
      (else
        (CallFunction|EnableTickCalc true)))))

(event EventBeginPlay
  (Utilities|FlowControl|Sequence
    (:then_0
      (Collision|AssignOnComponentBeginOverlap (EventDispatchers|CreateEvent :!event Custom|OnComponentBeginOverlap_Event))
      (Collision|BindEventtoOnComponentEndOverlap (EventDispatchers|CreateEvent :!event Custom|OnComponentEndOverlap_Event))
      (Variables|Default|SetOverlapping_LightTriggers (Collision|GetOverlappingActors "/Game/Blueprints/LightDetection/BP_BaseLightTrigger.BP_BaseLightTrigger_C" :!class /Script/Engine.PrimitiveComponent))
      (bind _value (CallFunction|IsinLight))
      (if _value
        (CallFunction|CheckLight)
        (CallFunction|EnableTickCalc true)))
    (:then_1
      ;[1 0.886 0] debug
      (bind _asbp_gm_base_debug (Utilities|Casting|CastToBP_GM_BaseDebug (Game|GetGameMode)))
      (EventDispatchers|AssignOnGMDebugChange _asbp_gm_base_debug (delegate Custom|On_GM_DebugChange_Event)))))

(event EventTick
  (params (DeltaSeconds :type Float%20%28single-precision%29))
  (if (Variables|Default|GetNo_Observers_Calc)
    (CallFunction|CheckLight)))

(fn CalcIlluminationValue
  (params (distance :type Float%20%28double-precision%29) (Target :type Object%20Object%20Reference))
  (LocalVariables|Setinput_distance distance)
  (bind _radius (Class|BPILightTrigger|GetAttenuationRadius(Message) Target))
  (LocalVariables|Setinput_radius _radius)
  (if (> (LocalVariables|Getinput_distance) (LocalVariables|Getinput_radius))
    (return 0.0)
    (else
      (bind _intensity (Class|BPILightTrigger|GetIntensity(Message) Target))
      (LocalVariables|Setinput_intensity _intensity)
      (bind _value (Class|BPILightTrigger|GetLightFalloffExponent(Message) Target))
      (LocalVariables|Setinput_falloff_exponent _value)
      (return (Utilities|IlluminationFormula (LocalVariables|Getinput_distance) (LocalVariables|Getinput_radius) (/ (LocalVariables|Getinput_falloff_exponent) 1.3))))))

(fn CheckLight
  (bind _returnvalue (Transformation|GetWorldLocation))
  (bind _returnvalue_2 (+ _returnvalue "0.000000,0.000000,-6.000000"))
  (Utilities|FlowControl|Sequence
    (:then_0
      (for _array_element (Variables|Default|GetOverlapping_LightTriggers)
        (bind _outhit (Collision|LineTraceByChannel (Transformation|GetActorLocation _array_element) (Transformation|GetWorldLocation) "TraceTypeQuery1" false 0 (select (Variables|Default|GetDebug) "ForOneFrame" "None") true "(R=0.145833,G=0.613801,B=1.000000,A=1.000000)" "(R=1.000000,G=0.000000,B=0.000000,A=1.000000)" 0.3))
        (if (not (.bBlockingHit (Collision|BreakHitResult _outhit)))
          (bind _illumination (CallFunction|CalcIlluminationValue (Math|Vector|Distance(Vector) (.TraceStart (Collision|BreakHitResult _outhit)) (.TraceEnd (Collision|BreakHitResult _outhit))) _array_element))
          (if (> _illumination (LocalVariables|Gethighest_illumination))
            (LocalVariables|Sethighest_illumination _illumination)
            (LocalVariables|Setlocal_distance (Math|Vector|Distance(Vector) (.TraceStart (Collision|BreakHitResult _outhit)) (.TraceEnd (Collision|BreakHitResult _outhit)))))))
      (Variables|Default|Setillumination_Value (LocalVariables|Gethighest_illumination))
      (bind _visibility (CallFunction|CalcVisibilityUsingDataTable (LocalVariables|Gethighest_illumination) "Default_Human"))
      (CallFunction|SetVisibilityValue _visibility))
    (:then_1
      (if (Variables|Default|GetDebug)
        ;[1 0.9144 0] Debug
        (Rendering|Debug|DrawDebugString _returnvalue (Utilities|String|Append "vis: " (Utilities|String|ToString(Float) (CallFunction|RemoveDecimalPart (Variables|Default|GetVisibility_Value) 10))) 0 "(R=1.000000,G=1.000000,B=1.000000,A=1.000000)")
        (Rendering|Debug|DrawDebugString _returnvalue_2 (Utilities|String|Append "dist: " (Utilities|String|ToString(Float) (CallFunction|RemoveDecimalPart (LocalVariables|Getlocal_distance) 10))) 0 "(R=0.000000,G=0.729663,B=1.000000,A=1.000000)")
        (Rendering|Debug|DrawDebugString (+ _returnvalue_2 "0.000000,0.000000,-6.000000") (Utilities|String|Append "ill:  " (Utilities|String|ToString(Float) (CallFunction|RemoveDecimalPart (LocalVariables|Gethighest_illumination) 10))) 0 "(R=0.838913,G=0.558058,B=1.000000,A=1.000000)")))))

(fn SetVisibilityValue
  (params (Visibility_Value :type Float%20%28double-precision%29))
  (Variables|Default|SetVisibility_Value Visibility_Value)
  (Default|CallOnChangeVisibility))

(fn IsinLight
  (return (not (Utilities|Array|IsEmpty (Variables|Default|GetOverlapping_LightTriggers)))))

(fn SetNoObserversCalc
  (params (new_val :type Boolean))
  (bind _output_get (Variables|Default|SetNo_Observers_Calc new_val))
  (if _output_get
    (Variables|Default|SetOverlapping_LightTriggers (Collision|GetOverlappingActors "/Game/Blueprints/LightDetection/BP_BaseLightTrigger.BP_BaseLightTrigger_C" :!class /Script/Engine.PrimitiveComponent))
    (bind _value (CallFunction|IsinLight))
    (if _value
      (Components|Tick|SetComponentTickEnabled true))
    (else
      (Components|Tick|SetComponentTickEnabled false))))

(fn EnableTickCalc
  (params (is_enable :type Boolean))
  (if (Variables|Default|GetNo_Observers_Calc)
    (Components|Tick|SetComponentTickEnabled is_enable)
    (else
      (Components|Tick|SetComponentTickEnabled false))))

(fn GetNoObserversCalc
  (return (Variables|Default|GetNo_Observers_Calc)))