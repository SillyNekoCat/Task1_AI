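; Rect light variant of a light-detection trigger, pairing a RectLight with a Box volume that can be shown through the game mode debug event.
; The construction script applies light parameters and fits the box in front of the light from attenuation radius and source size.
; Overridable-style getters expose intensity, radius plus smaller source side, and an angle-weighted falloff exponent.
; A half-sphere convex collision builder exists but never runs.
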(event EventBeginPlay
  (|CallParentFunction) ; This node is disabled and will not be called.\nDrag off pins to build functionality.
)

(event Collision|EventActorBeginOverlap
  (params (OtherActor :type Actor%20Object%20Reference))
  (|CallParentFunction OtherActor) ; This node is disabled and will not be called.\nDrag off pins to build functionality.
)

(event EventTick
  (params (DeltaSeconds :type Float%20%28single-precision%29))
  (|CallParentFunction DeltaSeconds) ; This node is disabled and will not be called.\nDrag off pins to build functionality.
)

(event EventOnGMDebugChangeEvent
  (params (debug :type Boolean))
  (|CallParentFunction debug)
  (CallFunction|SetVisibilityDebug (Variables|Default|GetBox) debug))

(fn ConstructionScript
  (bind _rectlight (Variables|Default|GetRectLight))
  (bind _attenuationradius (Variables|/Script/Engine.LocalLightComponent|GetAttenuationRadius _rectlight))
  (bind _returnvalue (/ _attenuationradius 2.0))
  (|CallParentFunction)
  (Utilities|FlowControl|Sequence
    (:then_0
      (Rendering|Components|Light|SetLightColor (Variables|Default|GetRectLight) (Variables|Default|GetLight_Color_param) true)
      (Rendering|Components|Light|SetIntensity (Variables|Default|GetRectLight) (Variables|Default|GetIntensity_param))
      (Rendering|Lighting|SetAttenuationRadius (Variables|Default|GetRectLight) (Variables|Default|GetAttenationRadius_param)))
    (:then_1
      (Components|Box|SetBoxExtent (Variables|Default|GetBox) (Math|Vector|MakeVector _returnvalue (+ _attenuationradius (Variables|/Script/Engine.RectLightComponent|GetSourceWidth _rectlight) 1.0) (+ _attenuationradius (Variables|/Script/Engine.RectLightComponent|GetSourceHeight _rectlight) 1.0)) true)
      (Transformation|SetRelativeLocation (Variables|Default|GetBox) (Math|Vector|MakeVector (+ _returnvalue 7.0) 0.0 0.0) false false))))

(fn GetAttenuationRadius
  (bind _rectlight (Variables|Default|GetRectLight))
  (bind _sourcewidth (Variables|/Script/Engine.RectLightComponent|GetSourceWidth _rectlight))
  (bind _sourceheight (Variables|/Script/Engine.RectLightComponent|GetSourceHeight _rectlight))
  (return (+ (Variables|/Script/Engine.LocalLightComponent|GetAttenuationRadius (Variables|Default|GetRectLight)) (Math|Float|SelectFloat _sourcewidth _sourceheight (< _sourcewidth _sourceheight)))))

(fn GetIntensity
  (return (Variables|/Script/Engine.LightComponentBase|GetIntensity (Variables|Default|GetRectLight))))

(fn GetLightFalloffExponent
  (params (optional_target_loc :type Vector :default "0, 0, 0"))
  (bind _rectlight (Variables|Default|GetRectLight))
  (return (* (- 1.0 (/ (CallFunction|InverseLerp (CallFunction|FindLookatDegrees (Math|Vector|GetForwardVector _rectlight) (Transformation|GetWorldLocation _rectlight) optional_target_loc) 0.0 9e+01) 2.0)) (LocalVariables|Getlight_fallof_exp))))

(fn MakeRectLightHalfSphere
  (params (dynamic_mesh :type Dynamic%20Mesh%20Object%20Reference))
  (bind _returnvalue (Class|KismetSystemLibrary|MakeLiteralInteger 16))
  (bind _returnvalue_2 (Class|GeometryScriptLibraryMeshPrimitiveFunctions|AppendSphereLatLong :TargetMesh dynamic_mesh :Radius (Variables|/Script/Engine.LocalLightComponent|GetAttenuationRadius (Variables|Default|GetRectLight)) :StepsPhi _returnvalue :StepsTheta _returnvalue :Debug 0))
  (bind _returnvalue_3 (Class|GeometryScriptLibraryMeshBooleanFunctions|ApplyMeshPlaneCut :TargetMesh _returnvalue_2 :Debug 0))
  (return _returnvalue_3))

(fn GetLightComp
  (return (Variables|Default|GetRectLight)))