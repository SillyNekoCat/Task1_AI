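; BP_BaseLightTrigger is a base Blueprint for light triggers in the light detection system.
; It declares getters for light component, intensity, attenuation radius, falloff exponent and outer angle, all returning placeholder values, apparently for child classes to override.
; On BeginPlay it binds to the debug-change event on BP_GM_BaseDebug to update its Debug flag.
; A helper toggles a scene component's visibility and hidden-in-game state for debug display.
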(event Custom|On_GM_DebugChange_Event
  (params (debug :type Boolean))
  ;[1 0.886 0] debug
  (Variables|Default|SetDebug debug))

(event EventBeginPlay
  (Utilities|FlowControl|Sequence
    (:then_1
      ;[1 0.886 0] debug
      (bind _asbp_gm_base_debug (Utilities|Casting|CastToBP_GM_BaseDebug (Game|GetGameMode)))
      (EventDispatchers|AssignOnGMDebugChange _asbp_gm_base_debug (delegate Custom|On_GM_DebugChange_Event)))))

(fn ConstructionScript)

(fn SetVisibilityDebug
  (params (target_scene_comp :type Scene%20Component%20Object%20Reference) (bNewVisibility :type Boolean))
  (Rendering|SetVisibility target_scene_comp bNewVisibility false)
  (Development|SetHiddeninGame target_scene_comp (not bNewVisibility) false))

(fn GetAttenuationRadius
  (return 0.0))

(fn GetIntensity
  (return 0.0))

(fn GetLightComp
  (return 0))

(fn GetLightFalloffExponent
  (params (optional_target_loc :type Vector :default "0, 0, 0"))
  (return 0.0))

(fn GetOuterAngle
  (return -1.0))