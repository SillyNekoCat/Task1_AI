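; BP_SpotLightTrigger is a spotlight light-detection trigger that pairs a configurable SpotLight with a capsule overlap volume.
; The construction script caps inner angle at outer, applies light parameters, then sizes and offsets the capsule to approximate the cone.
; Getters expose light properties, including a falloff exponent scaled by the target's angle between cone edges.
; Debug toggling shows the capsule; a Geometry Script cone-collision alternative is left unwired.
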(event EventBeginPlay
  (|CallParentFunction) ; This node is disabled and will not be called.\nDrag off pins to build functionality.
)

(event Collision|EventActorBeginOverlap
  (params (OtherActor :type Actor%20Object%20Reference))
  (|CallParentFunction OtherActor) ; This node is disabled and will not be called.\nDrag off pins to build functionality.
)

(event EventOnGMDebugChangeEvent
  (params (debug :type Boolean))
  (|CallParentFunction debug)
  (CallFunction|SetVisibilityDebug (Variables|Default|GetCapsule) debug))

(fn ConstructionScript
  (bind _spotlight (Variables|Default|GetSpotLight))
  (bind _outerconeangle_param (Variables|Default|GetOuterConeAngle_param))
  (bind _attenuationradius (Variables|/Script/Engine.LocalLightComponent|GetAttenuationRadius _spotlight))
  (|CallParentFunction)
  (Utilities|FlowControl|Sequence
    (:then_0
      (if (> (Variables|Default|GetInnerConeAngle_param) (Variables|Default|GetOuterConeAngle_param))
        (Rendering|Lighting|SetInnerConeAngle (Variables|Default|GetSpotLight) _outerconeangle_param)
        (bind _output_get (Variables|Default|SetInnerConeAngle_param _outerconeangle_param))
        (Rendering|Lighting|SetOuterConeAngle (Variables|Default|GetSpotLight) _output_get)
        (else
          (Rendering|Lighting|SetOuterConeAngle (Variables|Default|GetSpotLight) (Variables|Default|GetOuterConeAngle_param))
          (Rendering|Lighting|SetInnerConeAngle (Variables|Default|GetSpotLight) (Variables|Default|GetInnerConeAngle_param)))))
    (:then_1
      (Rendering|Lighting|SetAttenuationRadius (Variables|Default|GetSpotLight) (Variables|Default|GetAttenationRadius_param))
      (Rendering|Components|Light|SetIntensity (Variables|Default|GetSpotLight) (Variables|Default|GetIntensity_param))
      (Rendering|Components|Light|SetLightColor (Variables|Default|GetSpotLight) (Variables|Default|GetLight_Color_param) true))
    (:then_2
      (LocalVariables|Setcone_angle (Variables|/Script/Engine.SpotLightComponent|GetOuterConeAngle (Variables|Default|GetSpotLight)))
      (LocalVariables|Setlight_cone_radius (* (Variables|/Script/Engine.LocalLightComponent|GetAttenuationRadius (Variables|Default|GetSpotLight)) (Math|Trig|Sin(Degrees) (LocalVariables|Getcone_angle))))
      (Components|Capsule|SetCapsuleRadius (Variables|Default|GetCapsule) (LocalVariables|Getlight_cone_radius) true)
      (Components|Capsule|SetCapsuleHalfHeight (Variables|Default|GetCapsule) (- (+ (LocalVariables|Getlight_cone_radius) (/ (Variables|/Script/Engine.LocalLightComponent|GetAttenuationRadius (Variables|Default|GetSpotLight)) 2.0)) (+ (/ (LocalVariables|Getlight_cone_radius) 2.0) (/ (- (Variables|/Script/Engine.LocalLightComponent|GetAttenuationRadius (Variables|Default|GetSpotLight)) (* (Variables|/Script/Engine.LocalLightComponent|GetAttenuationRadius (Variables|Default|GetSpotLight)) (Math|Trig|Cos(Degrees) (LocalVariables|Getcone_angle)))) 2.0))) true)
      (Transformation|SetRelativeLocation (Variables|Default|GetCapsule) (Math|Vector|MakeVector (+ (- (+ (LocalVariables|Getlight_cone_radius) (/ (Variables|/Script/Engine.LocalLightComponent|GetAttenuationRadius (Variables|Default|GetSpotLight)) 2.0)) (+ (/ (LocalVariables|Getlight_cone_radius) 2.0) (/ (- (Variables|/Script/Engine.LocalLightComponent|GetAttenuationRadius (Variables|Default|GetSpotLight)) (* (Variables|/Script/Engine.LocalLightComponent|GetAttenuationRadius (Variables|Default|GetSpotLight)) (Math|Trig|Cos(Degrees) (LocalVariables|Getcone_angle)))) 2.0))) (Math|Float|SelectFloat (- (* (- (+ (LocalVariables|Getlight_cone_radius) (/ (Variables|/Script/Engine.LocalLightComponent|GetAttenuationRadius (Variables|Default|GetSpotLight)) 2.0)) (+ (/ (LocalVariables|Getlight_cone_radius) 2.0) (/ (- (Variables|/Script/Engine.LocalLightComponent|GetAttenuationRadius (Variables|Default|GetSpotLight)) (* (Variables|/Script/Engine.LocalLightComponent|GetAttenuationRadius (Variables|Default|GetSpotLight)) (Math|Trig|Cos(Degrees) (LocalVariables|Getcone_angle)))) 2.0))) (/ (- _attenuationradius (- (Variables|/Script/Engine.LocalLightComponent|GetAttenuationRadius (Variables|Default|GetSpotLight)) (* (Variables|/Script/Engine.LocalLightComponent|GetAttenuationRadius (Variables|Default|GetSpotLight)) (Math|Trig|Cos(Degrees) (LocalVariables|Getcone_angle))))) (- (+ (LocalVariables|Getlight_cone_radius) (/ (Variables|/Script/Engine.LocalLightComponent|GetAttenuationRadius (Variables|Default|GetSpotLight)) 2.0)) (+ (/ (LocalVariables|Getlight_cone_radius) 2.0) (/ (- (Variables|/Script/Engine.LocalLightComponent|GetAttenuationRadius (Variables|Default|GetSpotLight)) (* (Variables|/Script/Engine.LocalLightComponent|GetAttenuationRadius (Variables|Default|GetSpotLight)) (Math|Trig|Cos(Degrees) (LocalVariables|Getcone_angle)))) 2.0))))) (- (+ (LocalVariables|Getlight_cone_radius) (/ (Variables|/Script/Engine.LocalLightComponent|GetAttenuationRadius (Variables|Default|GetSpotLight)) 2.0)) (+ (/ (LocalVariables|Getlight_cone_radius) 2.0) (/ (- (Variables|/Script/Engine.LocalLightComponent|GetAttenuationRadius (Variables|Default|GetSpotLight)) (* (Variables|/Script/Engine.LocalLightComponent|GetAttenuationRadius (Variables|Default|GetSpotLight)) (Math|Trig|Cos(Degrees) (LocalVariables|Getcone_angle)))) 2.0)))) (- _attenuationradius (+ (* (- (+ (LocalVariables|Getlight_cone_radius) (/ (Variables|/Script/Engine.LocalLightComponent|GetAttenuationRadius (Variables|Default|GetSpotLight)) 2.0)) (+ (/ (LocalVariables|Getlight_cone_radius) 2.0) (/ (- (Variables|/Script/Engine.LocalLightComponent|GetAttenuationRadius (Variables|Default|GetSpotLight)) (* (Variables|/Script/Engine.LocalLightComponent|GetAttenuationRadius (Variables|Default|GetSpotLight)) (Math|Trig|Cos(Degrees) (LocalVariables|Getcone_angle)))) 2.0))) (/ (- _attenuationradius (- (Variables|/Script/Engine.LocalLightComponent|GetAttenuationRadius (Variables|Default|GetSpotLight)) (* (Variables|/Script/Engine.LocalLightComponent|GetAttenuationRadius (Variables|Default|GetSpotLight)) (Math|Trig|Cos(Degrees) (LocalVariables|Getcone_angle))))) (- (+ (LocalVariables|Getlight_cone_radius) (/ (Variables|/Script/Engine.LocalLightComponent|GetAttenuationRadius (Variables|Default|GetSpotLight)) 2.0)) (+ (/ (LocalVariables|Getlight_cone_radius) 2.0) (/ (- (Variables|/Script/Engine.LocalLightComponent|GetAttenuationRadius (Variables|Default|GetSpotLight)) (* (Variables|/Script/Engine.LocalLightComponent|GetAttenuationRadius (Variables|Default|GetSpotLight)) (Math|Trig|Cos(Degrees) (LocalVariables|Getcone_angle)))) 2.0))))) (- (Variables|/Script/Engine.LocalLightComponent|GetAttenuationRadius (Variables|Default|GetSpotLight)) (* (Variables|/Script/Engine.LocalLightComponent|GetAttenuationRadius (Variables|Default|GetSpotLight)) (Math|Trig|Cos(Degrees) (LocalVariables|Getcone_angle)))))) (<= (- (* (- (+ (LocalVariables|Getlight_cone_radius) (/ (Variables|/Script/Engine.LocalLightComponent|GetAttenuationRadius (Variables|Default|GetSpotLight)) 2.0)) (+ (/ (LocalVariables|Getlight_cone_radius) 2.0) (/ (- (Variables|/Script/Engine.LocalLightComponent|GetAttenuationRadius (Variables|Default|GetSpotLight)) (* (Variables|/Script/Engine.LocalLightComponent|GetAttenuationRadius (Variables|Default|GetSpotLight)) (Math|Trig|Cos(Degrees) (LocalVariables|Getcone_angle)))) 2.0))) (/ (- _attenuationradius (- (Variables|/Script/Engine.LocalLightComponent|GetAttenuationRadius (Variables|Default|GetSpotLight)) (* (Variables|/Script/Engine.LocalLightComponent|GetAttenuationRadius (Variables|Default|GetSpotLight)) (Math|Trig|Cos(Degrees) (LocalVariables|Getcone_angle))))) (- (+ (LocalVariables|Getlight_cone_radius) (/ (Variables|/Script/Engine.LocalLightComponent|GetAttenuationRadius (Variables|Default|GetSpotLight)) 2.0)) (+ (/ (LocalVariables|Getlight_cone_radius) 2.0) (/ (- (Variables|/Script/Engine.LocalLightComponent|GetAttenuationRadius (Variables|Default|GetSpotLight)) (* (Variables|/Script/Engine.LocalLightComponent|GetAttenuationRadius (Variables|Default|GetSpotLight)) (Math|Trig|Cos(Degrees) (LocalVariables|Getcone_angle)))) 2.0))))) (- (+ (LocalVariables|Getlight_cone_radius) (/ (Variables|/Script/Engine.LocalLightComponent|GetAttenuationRadius (Variables|Default|GetSpotLight)) 2.0)) (+ (/ (LocalVariables|Getlight_cone_radius) 2.0) (/ (- (Variables|/Script/Engine.LocalLightComponent|GetAttenuationRadius (Variables|Default|GetSpotLight)) (* (Variables|/Script/Engine.LocalLightComponent|GetAttenuationRadius (Variables|Default|GetSpotLight)) (Math|Trig|Cos(Degrees) (LocalVariables|Getcone_angle)))) 2.0)))) 0.0))) 0.0 0.0) false false))))

(fn GetAttenuationRadius
  (return (Variables|/Script/Engine.LocalLightComponent|GetAttenuationRadius (Variables|Default|GetSpotLight))))

(fn GetIntensity
  (return (Variables|/Script/Engine.LightComponentBase|GetIntensity (Variables|Default|GetSpotLight))))

(fn GetLightFalloffExponent
  (params (optional_target_loc :type Vector :default "0, 0, 0"))
  (bind _spotlight (Variables|Default|GetSpotLight))
  (bind _spotlight_2 (Variables|Default|GetSpotLight))
  (bind _spotlight_3 (Variables|Default|GetSpotLight))
  (bind _outerconeangle (Variables|/Script/Engine.SpotLightComponent|GetOuterConeAngle _spotlight))
  (bind _innerconeangle (Variables|/Script/Engine.SpotLightComponent|GetInnerConeAngle _spotlight_2))
  (if (Math|Float|NearlyEqual(Float) _outerconeangle _innerconeangle 0.01)
    (return (Variables|/Script/Engine.PointLightComponent|GetLightFalloffExponent (Variables|Default|GetSpotLight)))
    (else
      (return (* (CallFunction|InverseLerp (CallFunction|FindLookatDegrees (Math|Vector|GetForwardVector _spotlight_3) (Transformation|GetWorldLocation _spotlight_3) optional_target_loc) _outerconeangle _innerconeangle) (* (Variables|/Script/Engine.PointLightComponent|GetLightFalloffExponent (Variables|Default|GetSpotLight)) 1.3))))))

(fn MakeSpotlightCone
  (params (ToDynamicMesh :type Dynamic%20Mesh%20Object%20Reference))
  (bind _spotlight (Variables|Default|GetSpotLight))
  (bind _innerconeangle (Variables|/Script/Engine.SpotLightComponent|GetInnerConeAngle _spotlight))
  (LocalVariables|Setcone_angle (+ _innerconeangle (- (Variables|/Script/Engine.SpotLightComponent|GetOuterConeAngle (Variables|Default|GetSpotLight)) _innerconeangle)))
  (LocalVariables|Setradius (* (Variables|/Script/Engine.LocalLightComponent|GetAttenuationRadius (Variables|Default|GetSpotLight)) (Math|Trig|Sin(Degrees) (LocalVariables|Getcone_angle))))
  (LocalVariables|Setheight (* (Variables|/Script/Engine.LocalLightComponent|GetAttenuationRadius (Variables|Default|GetSpotLight)) (Math|Trig|Cos(Degrees) (LocalVariables|Getcone_angle))))
  (bind _returnvalue (Class|GeometryScriptLibraryMeshPrimitiveFunctions|AppendCone :TargetMesh ToDynamicMesh :Transform (Math|Transform|MakeTransform (Math|Vector|MakeVector 0.0 0.0 (* (LocalVariables|Getheight) -1.0))) :BaseRadius (LocalVariables|Getradius) :TopRadius 0.0 :Height (LocalVariables|Getheight) :RadialSteps 32 :HeightSteps 0 :Debug 0))
  ;[1 1 1] Select bottom vertex
  (bind (_selection _returnvalue_2) (Class|GeometryScriptLibraryMeshSelectionFunctions|SelectMeshElementsinSphere _returnvalue (Math|Vector|MakeVector 0.0 0.0 (Math|Float|MakeLiteralFloat (* (LocalVariables|Getheight) -1.0))) 5e+01 "Vertices" false))
  ;[1 1 1] Bottom Translate
  (bind _returnvalue_3 (Class|GeometryScriptLibraryMeshTransformFunctions|TranslateMeshSelection _returnvalue_2 _selection (Math|Vector|MakeVector 0.0 0.0 (* (Math|Float|Power (- (Variables|/Script/Engine.LocalLightComponent|GetAttenuationRadius (Variables|Default|GetSpotLight)) (LocalVariables|Getheight)) 1.2) -1.0)) 0))
  (return _returnvalue_3))

(fn GetOuterAngle
  (return (Variables|/Script/Engine.SpotLightComponent|GetOuterConeAngle (Variables|Default|GetSpotLight))))

(fn GetLightComp
  (return (Variables|Default|GetSpotLight)))