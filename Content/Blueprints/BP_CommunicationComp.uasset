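; Actor component that lets a pawn talk by playing a random talk montage on its skeletal mesh.
; TalkRequest accepts for player-controlled owners implementing BPI_Communication, while AI owners defer to their controller through that interface.
; Event_Talk starts the montage, or ends talk as failed if already talking.
; EndTalk clears the talking flag and fires OnEndTalking with success only when the montage completes.
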(event Custom|Event_Talk
  (bind _randomtalkmontages (Variables|Default|GetRandomTalkMontages))
  (if (Variables|Default|GetIsTalking)
    (CallFunction|EndTalk false)
    (else
      (Utilities|Array|Shuffle _randomtalkmontages)
      (Variables|Default|SetIsTalking true)
      (Animation|Montage|PlayMontage (Variables|Default|GetOwner_SkeletalMesh) (.OutItem (Utilities|Array|Random _randomtalkmontages))
        (:OnCompleted
          (CallFunction|EndTalk true))
        (:OnInterrupted
          (CallFunction|EndTalk false))))))

(event EventBeginPlay
  (bind _returnvalue (Components|GetOwner))
  (Variables|Default|SetOwner_SkeletalMesh (Actor|GetComponentbyClass _returnvalue "/Script/Engine.SkeletalMeshComponent"))
  (bind _aspawn (Utilities|Casting|CastToPawn _returnvalue))
  (Variables|Default|SetOwner_Pawn _aspawn))

(event EventTick
  (params (DeltaSeconds :type Float%20%28single-precision%29)))

(fn TalkRequest
  (params (request_owner :type Actor%20Object%20Reference))
  (bind _owner_pawn (Variables|Default|GetOwner_Pawn))
  (bind _returnvalue (AI|GetAIController _owner_pawn))
  (if (Pawn|IsPlayerControlled (Variables|Default|GetOwner_Pawn))
    (if (Utilities|DoesObjectImplementInterface (Components|GetOwner) "/Game/Blueprints/AI/BPI_Communication.BPI_Communication_C")
      (return true)
      (else
        _))
    (elif (Utilities|DoesObjectImplementInterface _returnvalue "/Game/Blueprints/AI/BPI_Communication.BPI_Communication_C") ; if ai
      (bind _result (Class|BPICommunication|RequestTalk(Message) _returnvalue request_owner))
      (return _result)
      (else
        _)))
  (return false))

(fn EndTalk
  (params (Success :type Boolean))
  (Variables|Default|SetIsTalking false)
  (Default|CallOnEndTalking Success))