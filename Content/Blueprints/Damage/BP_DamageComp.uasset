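; BP_DamageComp is a component that tracks its owner's health, damage intake and death.
; TakeDamage filters hits by team (only enemies unless ignored) and invulnerability (unless ignored), then subtracts damage, clamping health at zero.
; It broadcasts damage results for hits passing the team filter, and Death sets a dead flag and broadcasts source and last location.
; Health setters broadcast changes through dispatchers, which also fire with initial values on BeginPlay.
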(event EventBeginPlay
  (bind _self self)
  (Default|CallOnChangeCurrentHealth (Variables|Default|GetCurrent_Health) _self)
  (Default|CallOnChangeMaxHealth (Variables|Default|GetMax_Health) _self))

(event EventTick
  (params (DeltaSeconds :type Float%20%28single-precision%29)))

(fn TakeDamage
  (params (input_damage :type S%20Damage%20Structure))
  (bind (_ignore_team _instigator _damage_value _damage_loc _ignore_invul) (Utilities|Struct|BreakS_Damage input_damage))
  (bind _self self)
  (if _ignore_team
    _
    (else
      (bind _team_check_result (CallFunction|TeamCheck (Components|GetOwner) _instigator))
      (switch Utilities|FlowControl|Switch|SwitchonE_TeamCheck _team_check_result
        (:NewEnumerator2
          _))))
  (if _ignore_invul
    _
    (elif (Variables|Default|GetIs_Invul)
      (Default|CallOnTakeDamage false input_damage self)
      (return false)
      (else
        _)))
  (Utilities|FlowControl|Sequence
    (:then_0
      (LocalVariables|Setprev_curr_health (Variables|Default|GetCurrent_Health)))
    (:then_1
      ;[1 1 1] Apply damage
      (bind _is_changed (CallFunction|SetCurrentHealth (Math|Float|Max(Float) (- (Variables|Default|GetCurrent_Health) (.damage_value (Utilities|Struct|BreakS_Damage input_damage))) 0.0)))
      (LocalVariables|Setis_health_changed _is_changed))
    (:then_2
      ;[1 1 1] Death check
      (if (<= (Variables|Default|GetCurrent_Health) 0.0)
        (CallFunction|Death (.instigator (Utilities|Struct|BreakS_Damage input_damage)))))
    (:then_3
      ;[1 1 1] was damaged
      (if (LocalVariables|Getis_health_changed)
        (Default|CallOnTakeDamage true input_damage _self)
        (return true)
        (else
          (Default|CallOnTakeDamage false input_damage _self)
          (return false))))))

(fn Death
  (params (source :type Actor%20Object%20Reference))
  (Variables|Default|SetIs_Dead true)
  (Default|CallOnDeath source self (Transformation|GetActorLocation (Components|GetOwner))))

(fn SetCurrentHealth
  (params (new_value :type Float%20%28double-precision%29))
  (if (!= new_value (Variables|Default|GetCurrent_Health))
    (bind _output_get (Variables|Default|SetCurrent_Health new_value))
    (Default|CallOnChangeCurrentHealth _output_get self)
    (return true)
    (else
      (return false))))

(fn SetMaxHealth
  (params (new_value :type Float%20%28double-precision%29))
  (Utilities|FlowControl|Sequence
    (:then_0
      (if (!= new_value (Variables|Default|GetMax_Health))
        (bind _output_get (Variables|Default|SetMax_Health new_value))
        (Default|CallOnChangeMaxHealth _output_get self)))
    (:then_1
      (return (!= new_value (Variables|Default|GetMax_Health))))))

(fn GetIsDead
  (return (Variables|Default|GetIs_Dead)))