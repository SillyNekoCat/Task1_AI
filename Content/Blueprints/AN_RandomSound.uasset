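; Animation notify that plays a random sound during an animation and has the mesh's owning actor report a noise.
; It picks an entry from its Sounds array and plays it at the mesh component's world location.
; It then sends a MakeNoise message to the owner with configurable loudness, max range and tag.
; An empty array or invalid owner skips both sound and noise.
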(fn ReceivedNotify
  (params (MeshComp :type Skeletal%20Mesh%20Component%20Object%20Reference) (Animation :type Anim%20Sequence%20Base%20Object%20Reference) (EventReference :type Anim%20Notify%20Event%20Reference%20Structure%20%28by%20ref%29))
  (bind _returnvalue (Components|GetOwner MeshComp))
  (if (Utilities|Array|IsEmpty (Variables|Default|GetSounds))
    _
    (else
      (Utilities|IsValid _returnvalue
        (:Is%20Valid
          (Audio|PlaySoundatLocation (.OutItem (Utilities|Array|Random (Variables|Default|GetSounds))) (Transformation|GetWorldLocation MeshComp) "0, 0, 0" 1.0 1.0 0.0 0 0 0 0)
          (Class|BPINoise|MakeNoise(Message) _returnvalue (Variables|Default|GetNoise_Loudness) (Variables|Default|GetNoise_MaxRange) (Variables|Default|GetNoise_Tag))
          (return true))
        (:Is%20Not%20Valid
          _))))
  (return true))