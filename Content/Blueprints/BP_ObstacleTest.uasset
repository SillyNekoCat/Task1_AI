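; BP_ObstacleTest is a test obstacle that can become a physics object and damage what it hits while moving fast.
; SetActivation turns on physics simulation for the Cube when activated; deactivating changes nothing.
; On Box overlap, it checks that its speed exceeds a threshold and that the other actor's velocity differs enough from its own.
; It then sends team-ignoring damage to that actor's damage component.
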(event OnComponentBeginOverlap(Box)
  (params (OverlappedComponent :type Primitive%20Component%20Object%20Reference) (OtherActor :type Actor%20Object%20Reference) (OtherComp :type Primitive%20Component%20Object%20Reference) (OtherBodyIndex :type Integer) (bFromSweep :type Boolean) (SweepResult :type Hit%20Result%20Structure%20%28by%20ref%29))
  (bind _returnvalue (Transformation|GetVelocity))
  (bind _returnvalue_2 (Math|Float|MakeLiteralFloat 3e+02))
  (if (> (Math|Vector|VectorLength _returnvalue) _returnvalue_2)
    (if (not (Utilities|Operators|EqualEqual (Transformation|GetVelocity OtherActor) _returnvalue _returnvalue_2))
      (bind _comp (Class|BPIDamage|GetDamageComp(Message) OtherActor))
      (Utilities|IsValid _comp
        (:Is%20Valid
          (Default|TakeDamage _comp (Utilities|Struct|MakeS_Damage true self 1e+01 (Transformation|GetActorLocation))))))))

(event EventBeginPlay)

(event Collision|EventActorBeginOverlap
  (params (OtherActor :type Actor%20Object%20Reference)))

(event EventTick
  (params (DeltaSeconds :type Float%20%28single-precision%29)))

(fn ConstructionScript)

(fn SetActivation
  (params (is_active :type Boolean))
  (if is_active
    (Physics|SetSimulatePhysics (Variables|Default|GetCube) true)
    (return true)
    (else
      (return true))))