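; Ranged weapon Blueprint that fires a hitscan shot on AttackNotify, spawning a Niagara effect at the mesh's muzzle socket.
; The Visibility line trace starts at the owner's location and ends at the AI controller's focus actor, or straight ahead when there is none.
; The hit actor receives BaseDamage through an SDamage struct, and the game mode's debug flag toggles trace drawing.
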(event EventBeginPlay
  (|CallParentFunction) ; This node is disabled and will not be called.\nDrag off pins to build functionality.
)

(event Collision|EventActorBeginOverlap
  (params (OtherActor :type Actor%20Object%20Reference))
  (|CallParentFunction OtherActor) ; This node is disabled and will not be called.\nDrag off pins to build functionality.
)

(event EventTick
  (params (DeltaSeconds :type Float%20%28single-precision%29))
  (|CallParentFunction DeltaSeconds) ; This node is disabled and will not be called.\nDrag off pins to build functionality.
)

(event EventAttackNotify
  (bind _returnvalue (Utilities|Name|MakeLiteralName "Socket_End"))
  (bind _staticmesh (Variables|Default|GetStaticMesh))
  (bind _weapon_owner (Variables|Default|GetWeapon_Owner))
  (bind _weapon_owner_2 (Variables|Default|GetWeapon_Owner))
  (bind _returnvalue_2 (AI|GetAIController _weapon_owner_2))
  (bind _returnvalue_3 (Transformation|GetActorLocation _weapon_owner))
  (bind _returnvalue_4 (Class|AIController|GetFocusActor _returnvalue_2))
  (Utilities|FlowControl|Sequence
    (:then_0
      (Niagara|SpawnSystematLocation "/Game/Materials/NS_1.NS_1" (Transformation|GetSocketLocation _staticmesh _returnvalue) (Transformation|GetSocketRotation _staticmesh _returnvalue)))
    (:then_1
      (Utilities|IsValid _returnvalue_2
        (:Is%20Valid
          (Utilities|IsValid _returnvalue_4
            (:Is%20Valid
              (Variables|Default|SetTarget_Loc (Transformation|GetActorLocation _returnvalue_4))
              (Variables|Default|Settarget_shot true))
            (:Is%20Not%20Valid
              (Variables|Default|Settarget_shot false :!label _label))))
        (:Is%20Not%20Valid
          (goto _label)))
      (bind _debug (Class|BPIGMDebug|GetGlobalDebug(Message) (Game|GetGameMode)))
      (bind _outhit (Collision|LineTraceByChannel _returnvalue_3 (Math|Vector|SelectVector (Variables|Default|GetTarget_Loc) (+ _returnvalue_3 (* (Transformation|GetActorForwardVector _weapon_owner) 1.5e+03)) (Variables|Default|Gettarget_shot)) "TraceTypeQuery1" false (Utilities|Array|MakeArray (Variables|Default|GetWeapon_Owner) self) (select _debug "ForDuration" "None")))
      (CallFunction|Damage (.HitActor (Collision|BreakHitResult _outhit)) (Utilities|Struct|MakeS_Damage (Variables|Default|GetWeapon_Owner) (Variables|Default|GetBase_Damage) (Transformation|GetActorLocation) false)))))

(fn ConstructionScript
  (|CallParentFunction))