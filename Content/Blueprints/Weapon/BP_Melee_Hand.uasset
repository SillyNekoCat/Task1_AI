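; BP_Melee_Hand is a melee hand weapon that deals damage when its attack notify fires.
; AttackNotify runs a short forward sphere trace from the owner on the Visibility channel, with optional debug drawing.
; It sends a damage struct to the hit actor, using a fixed value instead of BaseDamage when that actor's AI controller reports either of two specific states.
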(event EventBeginPlay
  (|CallParentFunction))

(event Collision|EventActorBeginOverlap
  (params (OtherActor :type Actor%20Object%20Reference))
  (|CallParentFunction OtherActor) ; This node is disabled and will not be called.\nDrag off pins to build functionality.
)

(event EventTick
  (params (DeltaSeconds :type Float%20%28single-precision%29))
  (|CallParentFunction DeltaSeconds) ; This node is disabled and will not be called.\nDrag off pins to build functionality.
)

(event EventAttackNotify
  (bind _returnvalue (Math|Float|MakeLiteralFloat 3e+01))
  (bind _weapon_owner (Variables|Default|GetWeapon_Owner))
  (bind _returnvalue_2 (Transformation|GetActorForwardVector _weapon_owner))
  (bind _returnvalue_3 (Transformation|GetActorLocation _weapon_owner))
  (|CallParentFunction)
  (bind _outhit (Collision|SphereTraceByChannel (+ _returnvalue_3 (* _returnvalue_2 _returnvalue)) (+ _returnvalue_3 (* _returnvalue_2 6e+01)) _returnvalue "TraceTypeQuery1" false (Utilities|Array|MakeArray (Variables|Default|GetWeapon_Owner) self) (select (Variables|Default|GetDebug) "ForDuration" "None")))
  (bind _output_ai_state (Class|BPIAI|GetCurrentAIState(Message) (AI|GetAIController (.HitActor (Collision|BreakHitResult _outhit)))))
  (CallFunction|Damage (.HitActor (Collision|BreakHitResult _outhit)) (Utilities|Struct|MakeS_Damage (Variables|Default|GetWeapon_Owner) (Math|Float|SelectFloat 1e+01 (Variables|Default|GetBase_Damage) (or (Utilities|Enum|Equal(Enum) _output_ai_state "NewEnumerator4") (Utilities|Enum|Equal(Enum) _output_ai_state "NewEnumerator0"))) (Transformation|GetActorLocation) false)))

(fn ConstructionScript
  (|CallParentFunction))