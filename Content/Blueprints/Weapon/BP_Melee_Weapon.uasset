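; Melee weapon Blueprint that deals damage in front of its owner and shows that owner's team color.
; AttackNotify runs a short forward sphere trace on the Visibility channel, ignoring owner and weapon, and applies BaseDamage to the hit actor.
; SetWeaponOwner rebinds the owner's OnDeath event to hide the weapon, then runs SelectColor.
; SelectColor maps Blue or Red team tags to a dynamic material color, using a gate to skip untagged owners.
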(event Custom|On_Death_Event
  (params (source :type Actor%20Object%20Reference) (target_comp :type BP%20Damage%20Comp%20Object%20Reference) (last_target_loc :type Vector))
  (Rendering|SetActorHiddenInGame true))

(event EventBeginPlay
  (|CallParentFunction))

(event Collision|EventActorBeginOverlap
  (params (OtherActor :type Actor%20Object%20Reference))
  (|CallParentFunction OtherActor) ; This node is disabled and will not be called.\nDrag off pins to build functionality.
)

(event EventTick
  (params (DeltaSeconds :type Float%20%28single-precision%29))
  (|CallParentFunction DeltaSeconds) ; This node is disabled and will not be called.\nDrag off pins to build functionality.
)

(event EventAttackNotify
  (bind _returnvalue (Math|Float|MakeLiteralFloat 55.0))
  (bind _weapon_owner (Variables|Default|GetWeapon_Owner))
  (bind _returnvalue_2 (Transformation|GetActorForwardVector _weapon_owner))
  (bind _returnvalue_3 (Transformation|GetActorLocation _weapon_owner))
  (|CallParentFunction)
  (bind _outhit (Collision|SphereTraceByChannel (+ _returnvalue_3 (* _returnvalue_2 _returnvalue)) (+ _returnvalue_3 (* _returnvalue_2 85.0)) _returnvalue "TraceTypeQuery1" false (Utilities|Array|MakeArray (Variables|Default|GetWeapon_Owner) self) (select (Variables|Default|GetDebug) "ForDuration" "None")))
  (CallFunction|Damage (.HitActor (Collision|BreakHitResult _outhit)) (Utilities|Struct|MakeS_Damage (Variables|Default|GetWeapon_Owner) (Variables|Default|GetBase_Damage) (Transformation|GetActorLocation) false)))

(event EventSetWeaponOwner
  (params (input_weapon_owner :type Actor%20Object%20Reference))
  (bind _weapon_owner (Variables|Default|GetWeapon_Owner))
  (bind _weapon_owner_2 (Variables|Default|GetWeapon_Owner))
  (Utilities|FlowControl|Sequence
    (:then_0
      (Utilities|IsValid _weapon_owner
        (:Is%20Valid
          (bind _comp (Class|BPIDamage|GetDamageComp(Message) _weapon_owner))
          (EventDispatchers|UnbindEventfromOnDeath _comp (EventDispatchers|CreateEvent :!event Custom|On_Death_Event)))))
    (:then_1
      (|CallParentFunction input_weapon_owner)
      (CallFunction|SelectColor)
      (Utilities|IsValid _weapon_owner_2
        (:Is%20Valid
          (bind _comp_2 (Class|BPIDamage|GetDamageComp(Message) _weapon_owner_2))
          (EventDispatchers|AssignOnDeath _comp_2 (EventDispatchers|CreateEvent :!event Custom|On_Death_Event)))))))

(fn ConstructionScript
  (|CallParentFunction))

(fn SelectColor
  (bind _staticmesh (Variables|Default|GetStaticMesh))
  (Utilities|FlowControl|Sequence
    (:then_0
      (bind _tagcontainer (GameplayTags|GetOwnedGameplayTags (Variables|Default|GetWeapon_Owner) :!class /Script/GameplayTags.GameplayTagAssetInterface))
      (|SwitchGameplayTagContainer _tagcontainer
        (:Default
          (goto _label Close))
        (:%28GameplayTags=%28%28TagName="Team.Blue"%29%29%29
          (LocalVariables|SetColor "(R=0.001567,G=0.000000,B=1.000000,A=1.000000)"))
        (:%28GameplayTags=%28%28TagName="Team.Red"%29%29%29
          (LocalVariables|SetColor "(R=1.000000,G=0.000000,B=0.002574,A=1.000000)"))))
    (:then_1
      (Utilities|FlowControl|Gate false :!label _label
        (:Exit
          (bind _returnvalue (Rendering|Material|CreateDynamicMaterialInstance _staticmesh 0 (Rendering|Material|GetMaterial _staticmesh 0) "None" :!class /Script/Engine.PrimitiveComponent))
          (Rendering|Material|SetVectorParameterValue _returnvalue "Color" (LocalVariables|GetColor) :!class /Script/Engine.MaterialInstanceDynamic))))))