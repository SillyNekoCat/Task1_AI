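; Base weapon Blueprint that provides shared owner tracking, socket attachment, damage and montage getters, with empty attack-notify events, presumably for child weapons to override.
; Damage fetches the target's damage component through a message call and passes the amount to its TakeDamage.
; AttachWeapon snaps the weapon to Weapon_Socket on a given component.
; On BeginPlay it binds to BP_GM_BaseDebug's change event to keep its Debug value synced with the game mode.
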(event Custom|On_GM_DebugChange_Event
  (params (debug :type Boolean))
  ;[1 0.886 0] debug
  (Variables|Default|SetDebug debug))

(event EventBeginPlay
  (bind _returnvalue (Game|GetGameMode))
  (Utilities|FlowControl|Sequence
    (:then_1
      ;[1 0.886 0] debug
      (bind _asbp_gm_base_debug (Utilities|Casting|CastToBP_GM_BaseDebug _returnvalue))
      (EventDispatchers|AssignOnGMDebugChange _asbp_gm_base_debug (delegate Custom|On_GM_DebugChange_Event))
      (bind _debug (Class|BPIGMDebug|GetGlobalDebug(Message) _returnvalue))
      (Variables|Default|SetDebug _debug))))

(event Collision|EventActorBeginOverlap
  (params (OtherActor :type Actor%20Object%20Reference)))

(event EventSetWeaponOwner
  (params (input_weapon_owner :type Actor%20Object%20Reference))
  (Variables|Default|SetWeapon_Owner input_weapon_owner))

(event EventTick
  (params (DeltaSeconds :type Float%20%28single-precision%29)))

(event EventAttackNotify)

(event EventAttackNotifyStateBegin)

(event EventAttackNotifyStateEnd)

(event EventAttackNotifyStateTick)

(fn ConstructionScript)

(fn Damage
  (params (Target :type Object%20Object%20Reference) (input_damage :type S%20Damage%20Structure))
  (bind _comp (Class|BPIDamage|GetDamageComp(Message) Target))
  (Utilities|IsValid _comp
    (:Is%20Valid
      (Default|TakeDamage _comp input_damage))))

(fn AttachWeapon
  (params (attach_target :type Scene%20Component%20Object%20Reference))
  (Utilities|IsValid attach_target
    (:Is%20Valid
      (bind _returnvalue (Transformation|AttachComponentToComponent self attach_target "Weapon_Socket" "SnapToTarget" "SnapToTarget" "SnapToTarget" true))
      (return _returnvalue))
    (:Is%20Not%20Valid
      (return false))))

(fn GetEquipMontage
  (return (Variables|Default|GetWeapon_Equip_Montage)))

(fn GetHideMontage
  (return (Variables|Default|GetWeapon_Hide_Montage)))

(fn GetWeaponOwner
  (return (Variables|Default|GetWeapon_Owner)))

(fn GetWeaponMontages
  (return (Variables|Default|GetWeapon_Montages)))