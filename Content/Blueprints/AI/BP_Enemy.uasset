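; Enemy character that exposes combat, communication and movement controls, likely for its AI controller and other actors.
; Getters return the combat and communication components, while state queries and talk requests forward to the communication component.
; Movement speed is set either directly or by Idle/Walk/Run enum from DT_MovementValues, falling back to zero if the row is missing.
; Construction applies an overlay material to the mesh; a focus debug draw is left disconnected.
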(event EventTick
  (params (DeltaSeconds :type Float%20%28single-precision%29)))

(event EventBeginPlay)

(event EventSetValueMoveSpeed
  (params (move_speed_value :type Float%20%28double-precision%29))
  (Variables|/Script/Engine.CharacterMovementComponent|SetMaxWalkSpeed (Variables|Character|GetCharacterMovement) move_speed_value))

(fn ConstructionScript
  (Rendering|Material|SetOverlayMaterial (Variables|Character|GetMesh) "/Game/Materials/M_Overlay.M_Overlay" :!class /Script/Engine.MeshComponent))

(fn GetCombatComp
  (return (Variables|Components|GetBP_CombatComp)))

(fn GetCommunicationComp
  (return (Variables|Default|GetBP_CommunicationComp)))

(fn GetState
  (bind _state (Default|GetState (Variables|Default|GetBP_CommunicationComp)))
  (return _state))

(fn GetValuefromState
  (params (input_state :type E_AIState%20Enum :default "NewEnumerator7"))
  (bind (_vector_from_state _actor_from_state) (Default|GetValuefromState (Variables|Default|GetBP_CommunicationComp) input_state))
  (return _vector_from_state _actor_from_state))

(fn RequestTalk
  (params (request_owner :type Actor%20Object%20Reference))
  (bind _result (Default|TalkRequest (Variables|Default|GetBP_CommunicationComp) request_owner))
  (return _result))

(fn SetMoveSpeed
  (params (E_move_speed :type E_MoveSpeed%20Enum :default "NewEnumerator2"))
  (bind _returnvalue (Utilities|GetDataTableRow "/Game/Blueprints/Data/DT_MovementValues.DT_MovementValues" "Default")
    (:then
      (bind _output_get (Variables|/Script/Engine.CharacterMovementComponent|SetMaxWalkSpeed (Variables|Character|GetCharacterMovement) (Utilities|Select :Index E_move_speed :NewEnumerator2 (.Idle_Speed (Utilities|Struct|BreakS_MovementValues _returnvalue)) :NewEnumerator1 (.Walk_Speed (Utilities|Struct|BreakS_MovementValues _returnvalue)) :NewEnumerator0 (.Run_Speed (Utilities|Struct|BreakS_MovementValues _returnvalue)))))
      (return _output_get))
    (:RowNotFound
      (bind _output_get_2 (Variables|/Script/Engine.CharacterMovementComponent|SetMaxWalkSpeed (Variables|Character|GetCharacterMovement) 0.0))
      (return _output_get_2))))