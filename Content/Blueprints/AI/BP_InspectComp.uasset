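; AI component that holds a limited pool of inspect tokens, gating inspect behavior through a request and return scheme.
; RequestToken takes a token and reports success, or fails when none remain, while ReturnToken adds one back, clamped to the maximum.
; SetMaxTokens shifts available tokens by the change in maximum, preserving those in use.
; BeginPlay passes it the current maximum, leaving the available count unchanged.
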(event EventBeginPlay
  (CallFunction|SetMaxTokens (Variables|Default|GetMax_Inspect_Tokens)))

(event EventTick
  (params (DeltaSeconds :type Float%20%28single-precision%29)))

(fn RequestToken
  (if (<= (Variables|Default|GetInspect_Tokens) 0)
    (return false)
    (else
      (Utilities|FlowControl|Sequence
        (:then_0
          (Math|Integer|DecrementInt (Variables|Default|GetInspect_Tokens)))
        (:then_1
          (return true))))))

(fn ReturnToken
  (Variables|Default|SetInspect_Tokens (Math|Integer|Clamp(Integer) (+ (Variables|Default|GetInspect_Tokens) 1) 0 (Variables|Default|GetMax_Inspect_Tokens))))

(fn SetMaxTokens
  (params (input_value :type Integer))
  (Utilities|FlowControl|Sequence
    (:then_0
      (Variables|Default|SetInspect_Tokens (+ (Variables|Default|GetInspect_Tokens) (- input_value (Variables|Default|GetMax_Inspect_Tokens)))))
    (:then_1
      (Variables|Default|SetMax_Inspect_Tokens input_value))))