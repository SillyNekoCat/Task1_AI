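; Base AI controller that runs the enemy behavior tree and switches its blackboard AI state, with cooldown timers able to block states.
; Sight perception sorts targets by gameplay tags into enemies, allies for talk, and inspectables.
; Enemy shadow visibility scales detection distance and angle to trigger combat; a lost-target timer falls back to searching.
; Communication components relay alert states between allies in sight; hearing and damage handlers are unwired.
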(event OnPerceptionUpdated(AIPerception)
  (params (UpdatedActors :type Array%20of%20Actor%20Object%20References))
  (CallFunction|AllPerceptionUpdated UpdatedActors))

(event OnTargetPerceptionUpdated(AIPerception)
  (params (Actor :type Actor%20Object%20Reference) (Stimulus :type AI%20Stimulus%20Structure))
  (CallFunction|TargetPerceptionUpdated Actor Stimulus))

(event Custom|On_GM_DebugChange_Event
  (params (debug :type Boolean))
  ;[1 0.886 0] debug
  (Variables|Default|SetDebug debug))

(event Custom|EventTimer_CooldownInspectState
  (Utilities|Time|ClearandInvalidateTimerbyHandle (.Value (Utilities|Map|Find (Variables|Default|GetAIStates_InCooldown) "NewEnumerator1")))
  (Development|PrintString "end timer" true false "(R=0.201802,G=0.000000,B=1.000000,A=1.000000)"))

(event Custom|On_Owner_Destroy
  (params (DestroyedActor :type Actor%20Object%20Reference))
  (for _array_element (Variables|Default|GetEnemies_InSight)
    (bind _shadow_manager_comp (Class|BPIVisibility|GetShadowManager(Message) _array_element))
    (Default|DecrementObservers _shadow_manager_comp)))

(event Custom|EventTimer_CooldownCalmState
  (Utilities|Time|ClearandInvalidateTimerbyHandle (.Value (Utilities|Map|Find (Variables|Default|GetAIStates_InCooldown) "NewEnumerator4")))
  (Development|PrintString "end timer" true false "(R=0.201802,G=0.000000,B=1.000000,A=1.000000)"))

(event Custom|EventTimer_CooldownTalkState
  (Utilities|Time|ClearandInvalidateTimerbyHandle (.Value (Utilities|Map|Find (Variables|Default|GetAIStates_InCooldown) "NewEnumerator8")))
  (Development|PrintString "end timer" true false "(R=0.201802,G=0.000000,B=1.000000,A=1.000000)"))

(event EventBeginPlay
  (Utilities|FlowControl|Sequence
    (:then_0
      (AI|RunBehaviorTree "/Game/Blueprints/AI/BT_Enemy.BT_Enemy")
      (CallFunction|SetAIStateKey "NewEnumerator4"))
    (:then_1
      (Game|BindEventtoOnDestroyed (Pawn|GetControlledPawn) (EventDispatchers|CreateEvent :!event Custom|On_Owner_Destroy)))
    (:then_2
      ;[1 0.886 0] debug
      (bind _asbp_gm_base_debug (Utilities|Casting|CastToBP_GM_BaseDebug (Game|GetGameMode)))
      (EventDispatchers|AssignOnGMDebugChange _asbp_gm_base_debug (delegate Custom|On_GM_DebugChange_Event)))))

(event EventTick
  (params (DeltaSeconds :type Float%20%28single-precision%29))
  (Utilities|FlowControl|Sequence
    (:then_0
      (for _array_element (Variables|Default|GetEnemies_InSight)
        (bind _shadow_manager_comp (Class|BPIVisibility|GetShadowManager(Message) _array_element))
        (Default|PointsCheckLight _shadow_manager_comp)))
    (:then_1
      ;[1 0.886 0] debug
      (if (Variables|Default|GetDebug)
        (Rendering|Debug|DrawDebugString (Transformation|GetActorLocation (Pawn|GetControlledPawn)) (Utilities|String|EnumtoString (CallFunction|GetCurrentAIState)) 0 "(R=0.101020,G=0.395833,B=0.341558,A=1.000000)")))))

(event EventPossess
  (params (PossessedPawn :type Pawn%20Object%20Reference))
  (bind _comp (Class|BPICombat|GetCombatComp(Message) PossessedPawn))
  (Variables|Default|SetOwner_CombatComp _comp)
  (bind _comp_2 (Class|BPICommunication|GetCommunicationComp(Message) PossessedPawn))
  (Variables|Default|SetOwner_CommComp _comp_2))

(fn ConstructionScript)

(fn SetAIStateKey
  (params (Enum :type E_AIState%20Enum :default "NewEnumerator4"))
  (LocalVariables|Setinput_state Enum)
  (LocalVariables|Setcurrent_state (Utilities|Enum|ByteToEnumE_AIState (Class|BlackboardComponent|GetValueasEnum (Variables|Default|GetBlackboard) (Variables|Default|GetCurrentAIState_KeyName))))
  (if (not (.is_in_cooldown (CallFunction|IsStateinCooldown (LocalVariables|Getinput_state))))
    (if (Utilities|Enum|NotEqual(Enum) (LocalVariables|Getinput_state) (LocalVariables|Getcurrent_state))
      (Utilities|FlowControl|Sequence
        (:then_0
          ;[1 0.886 0] debug
          (if (Variables|Default|GetDebug)
            (if (Utilities|Enum|NotEqual(Enum) (Utilities|Enum|ByteToEnumE_AIState (Class|BlackboardComponent|GetValueasEnum (Variables|Default|GetBlackboard) (Variables|Default|GetCurrentAIState_KeyName))) (LocalVariables|Getinput_state))
              (Rendering|Debug|DrawDebugString (+ (Transformation|GetActorLocation (Pawn|GetControlledPawn)) "0.000000,0.000000,130.000000") (Utilities|String|EnumtoString (LocalVariables|Getinput_state)) 0 "(R=0.204698,G=0.401042,B=0.365168,A=1.000000)" 5.0))))
        (:then_1
          (AI|Components|Blackboard|SetValueasEnum (Variables|Default|GetBlackboard) (Variables|Default|GetPreviousAIState_KeyName) (LocalVariables|Getcurrent_state))
          (AI|Components|Blackboard|SetValueasEnum (Variables|Default|GetBlackboard) (Variables|Default|GetCurrentAIState_KeyName) (LocalVariables|Getinput_state)))))))

(fn SetLostTargetTimer
  (params (shadow_comp :type BP%20Shadow%20Manager%20Object%20Reference))
  (EventDispatchers|BindEventtoOnTimerLostTarget shadow_comp (EventDispatchers|CreateEvent :!event OnTimerLostTargetFunc))
  (Default|SetLostTargetTimer shadow_comp 1.0))

(fn SetCombatState
  (params (attack_target :type Actor%20Object%20Reference))
  (AI|Components|Blackboard|SetValueasObject (Variables|Default|GetBlackboard) (Variables|Default|GetAttackTarget_KeyName) attack_target)
  (CallFunction|SetAIStateKey "NewEnumerator3")
  (Default|CallOnInformAllyObservers :self (Variables|Default|GetOwner_CommComp) :state "NewEnumerator3" :actor attack_target))

(fn SetSearchEnemyTargetState
  (params (VectorValue :type Vector))
  (AI|Components|Blackboard|SetValueasVector (Variables|Default|GetBlackboard) (Variables|Default|GetInterestLocation_KeyName) VectorValue)
  (CallFunction|SetAIStateKey "NewEnumerator2")
  (Default|CallOnInformAllyObservers (Variables|Default|GetOwner_CommComp) "NewEnumerator2" VectorValue))

(fn SetInvestigateState
  (params (location :type Vector))
  (AI|Components|Blackboard|SetValueasVector (Variables|Default|GetBlackboard) (Variables|Default|GetInterestLocation_KeyName) location)
  (CallFunction|SetAIStateKey "NewEnumerator7")
  (CallFunction|SetAIStateKey "NewEnumerator1")
  (Default|CallOnInformAllyObservers (Variables|Default|GetOwner_CommComp) "NewEnumerator1" location))

(fn SetTalkState
  (params (actor :type Actor%20Object%20Reference))
  (AI|Components|Blackboard|SetValueasObject (Variables|Default|GetBlackboard) (Variables|Default|GetTalkTarget_KeyName) actor)
  (CallFunction|SetAIStateKey "NewEnumerator8"))

(fn SetInspectState
  (params (actor :type Actor%20Object%20Reference))
  (AI|Components|Blackboard|SetValueasObject (Variables|Default|GetBlackboard) (Variables|Default|GetInspectTarget_KeyName) actor)
  (CallFunction|SetAIStateKey "NewEnumerator0"))

(fn GetAttackTarget
  (bind _asactor (Utilities|Casting|CastToActor (AI|Components|Blackboard|GetValueasObject (Variables|Default|GetBlackboard) (Variables|Default|GetAttackTarget_KeyName)))
    (:then
      (return true _asactor))
    (:CastFailed
      (return false _asactor))))

(fn GetCurrentAIState
  (return (Utilities|Enum|ByteToEnumE_AIState (Class|BlackboardComponent|GetValueasEnum (Variables|Default|GetBlackboard) (Variables|Default|GetCurrentAIState_KeyName)))))

(fn CanSenseActor
  (params (Actor :type Actor%20Object%20Reference) (Sense :type E_Sense%20Enum :default "NewEnumerator3"))
  (bind _info (Class|AIPerceptionComponent|GetActorsPerception (Variables|Default|GetAIPerception) Actor))
  (for _array_element (.LastSensedStimuli (Utilities|Struct|BreakActorPerceptionBlueprintInfo _info))
    (bind _returnvalue (Class|AIPerceptionSystem|GetSenseClassforStimulus _array_element))
    (if (== _returnvalue (Utilities|Select :Index Sense :NewEnumerator3 0 :NewEnumerator2 "/Script/AIModule.AISense_Damage" :NewEnumerator0 "/Script/AIModule.AISense_Sight" :NewEnumerator1 "/Script/AIModule.AISense_Hearing"))
      (return _array_element (Utilities|Struct|BreakAIStimulus _array_element)))))

(fn HandleSight
  (params (actor :type Actor%20Object%20Reference))
  (LocalVariables|Setinput_actor actor)
  (bind _returnvalue (GameplayTags|HasAnyMatchingGameplayTags(Message) (LocalVariables|Getinput_actor) (Variables|/Game/Blueprints/BP_CombatComp.BP_CombatComp_C|GetEnemy_GameplayTags (Variables|Default|GetOwner_CombatComp))))
  (if _returnvalue ; is enemy
    _))

(fn HandleDamage
  (params (actor :type Actor%20Object%20Reference))
  (LocalVariables|Setinput_actor actor)
  (switch Utilities|FlowControl|Switch|SwitchonE_AIState (CallFunction|GetCurrentAIState)
    (:NewEnumerator7
      _)
    (:NewEnumerator4
      _)
    (:NewEnumerator8
      _)
    (:NewEnumerator0
      _)
    (:NewEnumerator1
      _)
    (:NewEnumerator2
      _))
  (CallFunction|SetCombatState (LocalVariables|Getinput_actor)))

(fn HandleHear
  (params (location :type Vector))
  (switch Utilities|FlowControl|Switch|SwitchonE_AIState (CallFunction|GetCurrentAIState)
    (:NewEnumerator7
      _)
    (:NewEnumerator4
      _)
    (:NewEnumerator8
      _)
    (:NewEnumerator0
      _)
    (:NewEnumerator1
      _))
  (CallFunction|SetInvestigateState location))

(fn TargetPerceptionUpdated
  (params (updated_target :type Actor%20Object%20Reference) (stimulus :type AI%20Stimulus%20Structure%20%28by%20ref%29))
  (bind _returnvalue (Class|AIPerceptionSystem|GetSenseClassforStimulus stimulus))
  (if (== _returnvalue "/Script/AIModule.AISense_Sight")
    (LocalVariables|Setis_successfully_sensed (.bSuccessfullySensed (Utilities|Struct|BreakAIStimulus (LocalVariables|GetStimulus))))
    (bind _returnvalue_2 (GameplayTags|HasAnyMatchingGameplayTags(Message) updated_target (Variables|/Game/Blueprints/BP_CombatComp.BP_CombatComp_C|GetEnemy_GameplayTags (Variables|Default|GetOwner_CombatComp))))
    (if _returnvalue_2 ; is enemy
      ;[1 1 1] Enemy
      (bind _shadow_manager_comp (Class|BPIVisibility|GetShadowManager(Message) updated_target))
      (LocalVariables|Settarget_shadow_comp _shadow_manager_comp)
      (if (LocalVariables|Getis_successfully_sensed)
        (CallFunction|AddEnemyinSight updated_target (LocalVariables|Gettarget_shadow_comp))
        (Utilities|IsValid (LocalVariables|Gettarget_shadow_comp)
          (:Is%20Valid
            (CallFunction|OnTotalVisibilityChangeFunc updated_target (LocalVariables|Gettarget_shadow_comp) (Default|GetTotalVisibility (LocalVariables|Gettarget_shadow_comp)) (Default|GetShadowValue (LocalVariables|Gettarget_shadow_comp)))
            (EventDispatchers|BindEventtoOnTotalVisibilityChange (LocalVariables|Gettarget_shadow_comp) (EventDispatchers|CreateEvent :!event OnTotalVisibilityChangeFunc))))
        (else
          (CallFunction|RemoveEnemyinSight updated_target (LocalVariables|Gettarget_shadow_comp))
          (Utilities|IsValid (LocalVariables|Gettarget_shadow_comp)
            (:Is%20Valid
              (EventDispatchers|UnbindEventfromOnTotalVisibilityChange (LocalVariables|Gettarget_shadow_comp) (EventDispatchers|CreateEvent :!event OnTotalVisibilityChangeFunc))
              (if (Utilities|Enum|Equal(Enum) (CallFunction|GetCurrentAIState) "NewEnumerator3")
                (CallFunction|SetLostTargetTimer (LocalVariables|Gettarget_shadow_comp)))))))
      (else
        (Utilities|FlowControl|Sequence ; not enemy
          (:then_0
            ;[1 1 1] Ally
            (bind _returnvalue_3 (GameplayTags|HasAnyMatchingGameplayTags(Message) updated_target (Variables|/Game/Blueprints/BP_CombatComp.BP_CombatComp_C|GetAlly_GameplayTags (Variables|Default|GetOwner_CombatComp))))
            (bind _output_get (LocalVariables|Setis_ally _returnvalue_3))
            (if _output_get ; is ally
              (bind _comp (Class|BPICommunication|GetCommunicationComp(Message) updated_target))
              (LocalVariables|Settarget_comm_comp _comp)
              (if (LocalVariables|Getis_successfully_sensed)
                (Utilities|IsValid (LocalVariables|Gettarget_comm_comp)
                  (:Is%20Valid
                    (EventDispatchers|BindEventtoOnInformAllyObservers (LocalVariables|Gettarget_comm_comp) (EventDispatchers|CreateEvent :!event OnInformAllyObserversFunc))))
                (else
                  (Utilities|IsValid (LocalVariables|Gettarget_comm_comp)
                    (:Is%20Valid
                      (EventDispatchers|UnbindEventfromOnInformAllyObservers (LocalVariables|Gettarget_comm_comp) (EventDispatchers|CreateEvent :!event OnInformAllyObserversFunc))))))))
          (:then_1
            ;[1 1 1] Inspect
            (switch Utilities|FlowControl|Switch|SwitchonE_AIState (CallFunction|GetCurrentAIState)
              (:NewEnumerator7
                _)
              (:NewEnumerator4
                _))
            (bind _comp_2 (Class|BPIInspect|GetInspectComp(Message) updated_target))
            (Utilities|IsValid _comp_2
              (:Is%20Valid
                (if (>= (Variables|/Game/Blueprints/BP_InspectComp.BP_InspectComp_C|GetTrigger_Distance _comp_2) (Math|Vector|Distance(Vector) (Transformation|GetActorLocation updated_target) (Transformation|GetActorLocation (Pawn|GetControlledPawn))))
                  (CallFunction|SetInspectState updated_target)))))
          (:then_2
            ;[1 1 1] Talk
            (if (not (.is_in_cooldown (CallFunction|IsStateinCooldown "NewEnumerator8")))
              (switch Utilities|FlowControl|Switch|SwitchonE_AIState (CallFunction|GetCurrentAIState)
                (:NewEnumerator7
                  _)
                (:NewEnumerator4
                  _))
              (if (LocalVariables|Getis_ally) ; is ally
                (bind _result (Class|BPICommunication|RequestTalk(Message) updated_target (Pawn|GetControlledPawn)))
                (if _result
                  (CallFunction|SetTalkState updated_target))))))))))

(fn AllPerceptionUpdated
  (params (Array :type Array%20of%20Actor%20Object%20References))
  (for _array_element Array
    (LocalVariables|Setlocal_array_actor _array_element)
    (Utilities|FlowControl|Sequence
      (:then_0
        ;[1 1 1] Sight
        (bind _successfully_sensed (CallFunction|CanSenseActor (LocalVariables|Getlocal_array_actor) "NewEnumerator0"))
        (if _successfully_sensed
          _))
      (:then_1
        (bind (_stimulus _successfully_sensed_2) (CallFunction|CanSenseActor (LocalVariables|Getlocal_array_actor) "NewEnumerator1"))
        (if _successfully_sensed_2
          _))
      (:then_2
        (bind _successfully_sensed_3 (CallFunction|CanSenseActor (LocalVariables|Getlocal_array_actor) "NewEnumerator2"))
        (if _successfully_sensed_3
          _)))))

(fn OnTotalVisibilityChangeFunc
  (params (actor :type Actor%20Object%20Reference) (shadow_comp :type BP%20Shadow%20Manager%20Object%20Reference) (new_total_visibility :type Float%20%28double-precision%29) (new_shadow_value :type Float%20%28double-precision%29))
  (bind _debug (Variables|Default|GetDebug))
  (LocalVariables|Settarget_actor actor)
  (LocalVariables|Setcomp shadow_comp)
  (LocalVariables|Settarget_visibility new_total_visibility)
  (LocalVariables|Settarget_distance (Math|Vector|Distance(Vector) (Transformation|GetActorLocation (LocalVariables|Gettarget_actor)) (Transformation|GetActorLocation (Pawn|GetControlledPawn))))
  (bind _angle (CallFunction|CalcAngleVisibilityUsingDataTable "Default_Human" (LocalVariables|Gettarget_visibility)))
  (LocalVariables|Setvisibility_angle _angle)
  (LocalVariables|Setcurrent_angle (CallFunction|AFindLookatDegrees (Pawn|GetControlledPawn) (LocalVariables|Gettarget_actor)))
  (bind _distance (CallFunction|CalcDistanceVisibilityUsingDataTable "Default_Human" (LocalVariables|Gettarget_visibility)))
  (LocalVariables|Setvisibility_distance _distance)
  (Utilities|FlowControl|Sequence
    (:then_0
      ;[1 0.886 0] debug
      (if _debug
        (|DebugVisibleAngle (LocalVariables|Getcurrent_angle) (LocalVariables|Getvisibility_angle) (LocalVariables|Getvisibility_distance) (LocalVariables|Gettarget_distance))))
    (:then_1
      (if (<= (LocalVariables|Gettarget_distance) (LocalVariables|Getvisibility_distance))
        (if (<= (LocalVariables|Getcurrent_angle) (LocalVariables|Getvisibility_angle))
          (Utilities|FlowControl|Sequence
            (:then_0
              (if _debug
                (Rendering|Debug|DrawDebugLine (Transformation|GetActorLocation (Pawn|GetControlledPawn)) (Transformation|GetActorLocation (LocalVariables|Gettarget_actor)) "(R=0.453885,G=0.927083,B=0.482986,A=1.000000)" 0.08 0.0)))
            (:then_1
              (Default|ClearLostTargerTimer (LocalVariables|Getcomp))
              ;[1 1 1] Activate Combat State
              (switch Utilities|FlowControl|Switch|SwitchonE_AIState (CallFunction|GetCurrentAIState)
                (:NewEnumerator7
                  _)
                (:NewEnumerator4
                  _)
                (:NewEnumerator8
                  _)
                (:NewEnumerator0
                  _)
                (:NewEnumerator1
                  _)
                (:NewEnumerator2
                  _))
              ;[1 1 1] Pick nearest attack target
              (bind (_succes _asactor) (CallFunction|GetAttackTarget))
              (if _succes
                (bind _actor (CallFunction|PickActorbyDistance true _asactor (LocalVariables|Gettarget_actor) (Pawn|GetControlledPawn)))
                (CallFunction|SetCombatState _actor)
                (else
                  (CallFunction|SetCombatState (LocalVariables|Gettarget_actor))))))
          (else
            (if (Utilities|Enum|Equal(Enum) (CallFunction|GetCurrentAIState) "NewEnumerator3") :!label _label
              (CallFunction|SetLostTargetTimer (LocalVariables|Getcomp)))))
        (else
          (goto _label))))))

(fn OnTimerLostTargetFunc
  (params (actor :type Actor%20Object%20Reference) (comp :type BP%20Shadow%20Manager%20Object%20Reference))
  (bind (_succes _asactor) (CallFunction|GetAttackTarget))
  (if _succes
    (if (== _asactor actor)
      (EventDispatchers|UnbindEventfromOnTimerLostTarget comp (EventDispatchers|CreateEvent :!event OnTimerLostTargetFunc))
      (Utilities|FlowControl|Sequence
        (:then_0
          (CallFunction|SetSearchEnemyTargetState (Transformation|GetActorLocation actor)))))))

(fn OnInformAllyObserversFunc
  (params (state :type E_AIState%20Enum :default "NewEnumerator7") (loc :type Vector) (actor :type Actor%20Object%20Reference))
  (if (not (Utilities|Enum|Equal(Enum) (CallFunction|GetCurrentAIState) state))
    (switch Utilities|FlowControl|Switch|SwitchonE_AIState state
      (:NewEnumerator1
        (CallFunction|SetInvestigateState loc))
      (:NewEnumerator2
        (CallFunction|SetSearchEnemyTargetState loc))
      (:NewEnumerator3
        (CallFunction|SetCombatState actor)))))

(fn AddEnemyinSight
  (params (enemy :type Actor%20Object%20Reference%20%28by%20ref%29) (shadow_comp :type BP%20Shadow%20Manager%20Object%20Reference))
  (Utilities|Array|AddUnique (Variables|Default|GetEnemies_InSight) enemy)
  (Utilities|IsValid shadow_comp
    (:Is%20Valid
      (Default|IncrementObservers shadow_comp))))

(fn RemoveEnemyinSight
  (params (enemy :type Actor%20Object%20Reference%20%28by%20ref%29) (shadow_comp :type BP%20Shadow%20Manager%20Object%20Reference))
  (Utilities|Array|RemoveItem (Variables|Default|GetEnemies_InSight) enemy)
  (Utilities|IsValid shadow_comp
    (:Is%20Valid
      (Default|DecrementObservers shadow_comp))))

(fn IsStateinCooldown
  (params (Key :type E_AIState%20Enum :default "NewEnumerator7"))
  (bind _aistates_incooldown (Variables|Default|GetAIStates_InCooldown))
  (bind _value (Utilities|Map|Find _aistates_incooldown Key))
  (return (Utilities|Time|IsValidTimerHandle _value) _value))

(fn SetTimerCooldownState
  (params (State :type E_AIState%20Enum%20%28by%20ref%29 :default "NewEnumerator7") (Time :type Float%20%28single-precision%29))
  (switch Utilities|FlowControl|Switch|SwitchonE_AIState State
    (:NewEnumerator4
      (bind _returnvalue (Utilities|Time|SetTimerbyEvent (EventDispatchers|CreateEvent :!event Custom|EventTimer_CooldownCalmState) Time))
      (Utilities|Map|Add (Variables|Default|GetAIStates_InCooldown) State _returnvalue))
    (:NewEnumerator8
      (bind _returnvalue_2 (Utilities|Time|SetTimerbyEvent (EventDispatchers|CreateEvent :!event Custom|EventTimer_CooldownTalkState) Time))
      (Utilities|Map|Add (Variables|Default|GetAIStates_InCooldown) State _returnvalue_2))
    (:NewEnumerator0
      (bind _returnvalue_3 (Utilities|Time|SetTimerbyEvent (EventDispatchers|CreateEvent :!event Custom|EventTimer_CooldownInspectState) Time))
      (Utilities|Map|Add (Variables|Default|GetAIStates_InCooldown) State _returnvalue_3)))
  (Development|PrintString (Utilities|String|Append (Utilities|String|EnumtoString State) "# " (Utilities|String|ToString(Float) Time)) true false "(R=0.000000,G=0.660000,B=1.000000,A=1.000000)" Time))

(fn GetCommunicationComp
  (return (Variables|Default|GetOwner_CommComp)))

(fn RequestTalk
  (params (request_owner :type Actor%20Object%20Reference))
  (switch Utilities|FlowControl|Switch|SwitchonE_AIState (CallFunction|GetCurrentAIState)
    (:NewEnumerator7
      (if (.is_in_cooldown (CallFunction|IsStateinCooldown "NewEnumerator8")) :!label _label
        _
        (else
          (CallFunction|SetTalkState request_owner)
          (Development|PrintString "request talk true" true true "(R=0.000000,G=1.000000,B=0.038456,A=1.000000)")
          (return true))))
    (:NewEnumerator4
      (goto _label))
    (:NewEnumerator8
      _)
    (:NewEnumerator0
      _)
    (:NewEnumerator1
      _)
    (:NewEnumerator2
      _)
    (:NewEnumerator3
      _)
    (:NewEnumerator5
      _))
  (Development|PrintString "request talk false" true true "(R=1.000000,G=0.000000,B=0.053658,A=1.000000)")
  (return false))