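; Patrol component for AI that tracks an index into a list of patrol points and can vary the route over time.
; Index increments follow a signed direction, wrapping at either end and optionally reversing.
; A self-restarting random-interval timer shuffles points, reverses direction or randomly picks either, using caller-supplied settings or component defaults.
; The debug game mode's change event toggles Tick, which draws timer and method text above the owner.
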(event Custom|On_GM_DebugChange_Event
  (params (debug :type Boolean))
  ;[1 0.886 0] debug
  (bind _output_get (Variables|Default|SetDebug debug))
  (Components|Tick|SetComponentTickEnabled _output_get))

(event Custom|TimerEvent_IntervalRouteChange
  (bind _route_change_method (Variables|Patrol|GetRoute_Change_Method))
  (bind _input_routechangemethod (Variables|Default|GetInput_RouteChangeMethod))
  (bind _input_routechangemethod_2 (Variables|Default|GetInput_RouteChangeMethod))
  (bind _route_change_method_2 (Variables|Patrol|GetRoute_Change_Method))
  (bind _returnvalue (Utilities|Enum|Equal(Enum) _input_routechangemethod_2 "NewEnumerator4"))
  (bind _returnvalue_2 (select _returnvalue _route_change_method_2 _input_routechangemethod))
  ;[1 1 1] interval route changes
  (if (Variables|Patrol|GetIs_IntervalRouteChange_Active)
    (if (Math|Boolean|ANDBoolean (Utilities|Enum|NotEqual(Enum) _route_change_method "NewEnumerator3") (Utilities|Enum|NotEqual(Enum) _route_change_method "NewEnumerator4") (Utilities|Enum|NotEqual(Enum) (Variables|Default|GetInput_RouteChangeMethod) "NewEnumerator3"))
      (CallFunction|ChangePatrolRoute _returnvalue_2)
      (CallFunction|StartIntervalRouteChange _returnvalue_2 (Variables|Patrol|Getresult_MinInterv_ChangeRoute) (Variables|Patrol|Getresult_MaxInterv_ChangeRoute)))))

(event Custom|Increment_PatrolPointIndex
  ;[1 1 1] Increment_PatrolPointIndex
  (Variables|Patrol|SetPatrolPointIndex (+ (Variables|Patrol|GetPatrolPointIndex) (Variables|Patrol|GetDirection)))
  (if (> (Variables|Patrol|GetPatrolPointIndex) (Utilities|Array|LastIndex (Variables|Patrol|GetPatrol_Points)))
    (Variables|Patrol|SetPatrolPointIndex 0) ; Reset index
    (if (Variables|Patrol|GetIsReverseDirectionAtEnd) :!label _label
      (CallFunction|ReversePatrolRouteDirection))
    (elif (< (Variables|Patrol|GetPatrolPointIndex) 0)
      (Variables|Patrol|SetPatrolPointIndex (Utilities|Array|LastIndex (Variables|Patrol|GetPatrol_Points))) ; Reset index
      (goto _label))))

(event Custom|Start_Interval_Route_Change
  (params (Patrol_Route_Change_Method :type E_PatrolRoute_Change%20Enum :default "NewEnumerator2") (MinInterv_RouteChange :type Float%20%28double-precision%29) (MaxInterv_RouteChange :type Float%20%28double-precision%29))
  (bind _route_change_method (Variables|Patrol|GetRoute_Change_Method))
  ;[1 1 1] interval route changes
  (Variables|Default|SetInput_RouteChangeMethod Patrol_Route_Change_Method)
  (if (Math|Boolean|ANDBoolean (Utilities|Enum|NotEqual(Enum) _route_change_method "NewEnumerator3") (Utilities|Enum|NotEqual(Enum) _route_change_method "NewEnumerator4") (Utilities|Enum|NotEqual(Enum) (Variables|Default|GetInput_RouteChangeMethod) "NewEnumerator3"))
    (bind _interval (CallFunction|ValidRandInterval MinInterv_RouteChange MaxInterv_RouteChange))
    (bind _returnvalue (Utilities|Time|SetTimerbyEvent (delegate Custom|TimerEvent_IntervalRouteChange) _interval))
    (Variables|Patrol|SetRouteChange_TimerHandle _returnvalue)
    (Variables|Patrol|SetIs_IntervalRouteChange_Active true)))

(event EventBeginPlay
  (Utilities|FlowControl|Sequence
    (:then_1
      ;[1 0.886 0] debug
      (bind _asbp_gm_base_debug (Utilities|Casting|CastToBP_GM_BaseDebug (Game|GetGameMode)))
      (EventDispatchers|AssignOnGMDebugChange _asbp_gm_base_debug (delegate Custom|On_GM_DebugChange_Event)))))

(event EventTick
  (params (DeltaSeconds :type Float%20%28single-precision%29))
  (CallFunction|DEBUG1))

(fn ValidRandInterval
  (params (min_interval :type Float%20%28double-precision%29) (max_interval :type Float%20%28double-precision%29))
  (if (or (<= min_interval 0.0) (<= max_interval 0.0))
    ;[1 1 1] if < 0 use editable values of this component
    (Variables|Patrol|Setresult_MinInterv_ChangeRoute (Variables|Patrol|GetMinInterv_RouteChange))
    (Variables|Patrol|Setresult_MaxInterv_ChangeRoute (Variables|Patrol|GetMaxInterv_RouteChange))
    (else
      (Variables|Patrol|Setresult_MinInterv_ChangeRoute min_interval)
      (Variables|Patrol|Setresult_MaxInterv_ChangeRoute max_interval)))
  (return (Math|Random|RandomFloatinRange (Variables|Patrol|Getresult_MinInterv_ChangeRoute) (Variables|Patrol|Getresult_MaxInterv_ChangeRoute))))

(fn ChangePatrolRoute
  (params (route_changing_method :type E_PatrolRoute_Change%20Enum :default "NewEnumerator3"))
  (switch Utilities|FlowControl|Switch|SwitchonE_PatrolRoute_Change (Utilities|Select :Index route_changing_method :NewEnumerator3 "NewEnumerator3" :NewEnumerator4 (Variables|Patrol|GetRoute_Change_Method) :NewEnumerator2 "NewEnumerator2" :NewEnumerator0 "NewEnumerator0" :NewEnumerator1 "NewEnumerator1")
    (:NewEnumerator2
      (switch int (Math|Random|RandomIntegerinRange 1 2)
        (:1
          (Utilities|Array|Shuffle (Variables|Patrol|GetPatrol_Points) :!label _label))
        (:2
          (CallFunction|ReversePatrolRouteDirection :!label _label_2))))
    (:NewEnumerator0
      (goto _label))
    (:NewEnumerator1
      (goto _label_2))))

(fn GetIsIntervalRouteChangeActive
  (return (Variables|Patrol|GetIs_IntervalRouteChange_Active)))

(fn ReversePatrolRouteDirection
  (Variables|Patrol|SetDirection (* (Variables|Patrol|GetDirection) -1)))

(fn StopRouteChange
  (Utilities|Time|ClearandInvalidateTimerbyHandle (Variables|Patrol|GetRouteChange_TimerHandle))
  (Variables|Patrol|SetIs_IntervalRouteChange_Active false))

(fn DEBUG1
  (bind _returnvalue (Components|GetOwner))
  (bind _returnvalue_2 (Transformation|GetActorLocation _returnvalue))
  (bind _returnvalue_3 (+ _returnvalue_2 "0.000000,0.000000,120.000000"))
  (Rendering|Debug|DrawDebugString _returnvalue_3 (Utilities|String|Append "                Min:" (Utilities|String|ToString(Float) (Variables|Patrol|Getresult_MinInterv_ChangeRoute)) "| Max:" (Utilities|String|ToString(Float) (Variables|Patrol|Getresult_MaxInterv_ChangeRoute)) "  # " "Route Change Timer: " (Utilities|String|ToString(Float) (Utilities|Time|GetTimerRemainingTimebyHandle (Variables|Patrol|GetRouteChange_TimerHandle)))) 0 "(R=1.000000,G=1.000000,B=1.000000,A=1.000000)")
  (Rendering|Debug|DrawDebugString (+ _returnvalue_3 "0.000000,0.000000,25.000000") (Utilities|String|Append "                Route Change Method: " (Utilities|String|EnumtoString (select (Utilities|Enum|Equal(Enum) (Variables|Default|GetInput_RouteChangeMethod) "NewEnumerator4") (Variables|Patrol|GetRoute_Change_Method) (Variables|Default|GetInput_RouteChangeMethod)))) 0 "(R=1.000000,G=1.000000,B=1.000000,A=1.000000)"))