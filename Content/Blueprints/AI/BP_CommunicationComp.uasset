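; BP_CommunicationComp is a pawn component that handles talking between characters and tracks which actors have joined a status.
; Event_Talk plays a random montage on the owner's skeletal mesh, or ends talk if already talking, then broadcasts success or failure through EndTalk.
; RequestTalk forwards requests to the pawn when player-controlled, otherwise to its AI controller, returning false without one.
; Helper functions add, check and clear the joined-actor list.
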(event Custom|Event_Talk
  (bind _randomtalkmontages (Variables|Default|GetRandomTalkMontages))
  (if (Variables|Default|GetIsTalking)
    (CallFunction|EndTalk false)
    (else
      (Utilities|Array|Shuffle _randomtalkmontages)
      (Variables|Default|SetIsTalking true)
      (Animation|Montage|PlayMontage (Variables|Default|GetOwner_SkeletalMesh) (.OutItem (Utilities|Array|Random _randomtalkmontages)) (Math|Float|MakeLiteralFloat 2.0) ; talk montage
        (:OnCompleted
          (CallFunction|EndTalk true))
        (:OnInterrupted
          (CallFunction|EndTalk false))))))

(event EventBeginPlay
  (bind _returnvalue (Components|GetOwner))
  (Variables|Default|SetOwner_SkeletalMesh (Actor|GetComponentbyClass _returnvalue "/Script/Engine.SkeletalMeshComponent"))
  (bind _aspawn (Utilities|Casting|CastToPawn _returnvalue))
  (Variables|Default|SetOwner_Pawn _aspawn))

(event EventTick
  (params (DeltaSeconds :type Float%20%28single-precision%29)))

(fn EndTalk
  (params (Success :type Boolean))
  (Variables|Default|SetIsTalking false)
  (Default|CallOnEndTalking Success))

(fn IsActorJoinedtoStatus
  (params (input_actor :type Actor%20Object%20Reference%20%28by%20ref%29))
  (return (Utilities|Array|ContainsItem (Variables|Default|GetActors_Joined_toStatus%20) input_actor)))

(fn ClearActorsJoinedtoStatus
  (Utilities|Array|Clear (Variables|Default|GetActors_Joined_toStatus%20)))

(fn AddActorsJoinedtoStatus
  (params (input_actor :type Actor%20Object%20Reference%20%28by%20ref%29))
  (Utilities|Array|AddUnique (Variables|Default|GetActors_Joined_toStatus%20) input_actor))

(fn GetCommunicationComp
  (return self))

(fn RequestTalk
  (params (request_owner :type Actor%20Object%20Reference))
  (bind _owner_pawn (Variables|Default|GetOwner_Pawn))
  (bind _returnvalue (AI|GetAIController _owner_pawn))
  (if (Pawn|IsPlayerControlled (Variables|Default|GetOwner_Pawn))
    (bind _result (Class|BPICommunication|RequestTalk(Message) (Variables|Default|GetOwner_Pawn) request_owner))
    (return _result)
    (else
      (Utilities|IsValid _returnvalue
        (:Is%20Valid
          (bind _result_2 (Class|BPICommunication|RequestTalk(Message) _returnvalue request_owner))
          (return _result_2))
        (:Is%20Not%20Valid
          (return false))))))