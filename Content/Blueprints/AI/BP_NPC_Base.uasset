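; Base NPC character that runs its default behavior tree when an AI controller takes it over.
; It exposes combat, damage, patrol and communication components through getters, with placeholder returns for AI state and target queries.
; Movement speed comes from a data table by speed enum, and crowd avoidance toggles by swapping avoidance group masks.
; Damage-component death ragdolls the mesh, hides the HP widget, removes the capsule and sets a short lifespan.
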(event Custom|On_Death_Event
  (params (source :type Actor%20Object%20Reference) (target_comp :type BP%20Damage%20Comp%20Object%20Reference) (last_target_loc :type Vector))
  (bind _mesh (Variables|Character|GetMesh))
  ;[1 1 1] Death
  (Utilities|FlowControl|Sequence
    (:then_0
      (Collision|SetCollisionEnabled _mesh "QueryAndPhysics")
      (Physics|SetSimulatePhysics _mesh true))
    (:then_1
      (Rendering|SetVisibility (Variables|Default|GetBP_HP_WidgetComp) false false))
    (:then_2
      (Components|DestroyComponent (Variables|Default|GetCapsuleComponent))
      (Actor|SetLifeSpan 4.0))))

(event EventTick
  (params (DeltaSeconds :type Float%20%28single-precision%29)))

(event EventBeginPlay
  (Utilities|FlowControl|Sequence
    (:then_0
      (Variables|Default|SetDefault%20Avoidance%20Group (Variables|/Script/Engine.CharacterMovementComponent|GetAvoidanceGroup (Variables|Character|GetCharacterMovement))))
    (:then_1
      (EventDispatchers|AssignOnDeath (Variables|Default|GetBP_DamageComp) (EventDispatchers|CreateEvent :!event Custom|On_Death_Event)))))

(event EventSetValueMoveSpeed
  (params (move_speed_value :type Float%20%28double-precision%29))
  (Variables|/Script/Engine.CharacterMovementComponent|SetMaxWalkSpeed (Variables|Character|GetCharacterMovement) move_speed_value))

(event EventSetAvoidance
  (params (is_enabled :type Boolean))
  ;[1 1 1] Avoidance control
  (if is_enabled
    (Class|CharacterMovementComponent|SetAvoidanceGroupMask (Variables|Character|GetCharacterMovement) (Variables|Default|GetDefault%20Avoidance%20Group))
    (Class|BPIAI|UpdateCrowdAgent(Message) (AI|GetAIController (Pawn|GetController)))
    (else
      (Variables|Default|SetDefault%20Avoidance%20Group (Variables|/Script/Engine.CharacterMovementComponent|GetAvoidanceGroup (Variables|Character|GetCharacterMovement)))
      (Class|CharacterMovementComponent|SetAvoidanceGroupMask (Variables|Character|GetCharacterMovement) (Utilities|Struct|MakeNavAvoidanceMask false false))
      (Class|BPIAI|UpdateCrowdAgent(Message) (AI|GetAIController (Pawn|GetController))))))

(event EventMakeNoise
  (params (Noise_Loudness :type Float%20%28double-precision%29) (Noise_MaxRange :type Float%20%28double-precision%29) (Noise_Tag :type Name :default "None"))
  ;[1 1 1] Noise
  (Class|Actor|MakeNoise Noise_Loudness self (Transformation|GetActorLocation) Noise_MaxRange Noise_Tag))

(event EventControllerChanged
  (params (OldController :type Controller%20Object%20Reference) (NewController :type Controller%20Object%20Reference))
  ;[1 1 1] Init BT
  (if (Utilities|IsValid NewController)
    (if (not (Class|Controller|IsPlayerController NewController))
      (AI|RunBehaviorTree (AI|GetAIController self) (Variables|Default|GetBT_Default)))))

(fn ConstructionScript)

(fn GetIsAIStateinCooldown
  (params (state :type E_AIState%20Enum :default "NewEnumerator7"))
  (return false))

(fn GetPrevAIState
  (return "NewEnumerator7"))

(fn GetCurrentAIState
  (return "NewEnumerator7"))

(fn GetInterestLocation
  (return "0, 0, 0"))

(fn GetAttackTarget
  (return 0))

(fn GetCombatComp
  (return (Variables|Components|GetBP_CombatComp)))

(fn GetCommunicationComp
  (return (Variables|Default|GetBP_CommunicationComp)))

(fn GetDamageComp
  (return (Variables|Default|GetBP_DamageComp)))

(fn GetMoveSpeed
  (return (Class|MovementComponent|GetMaxSpeed (Variables|Character|GetCharacterMovement))))

(fn GetPatrolComp
  (return (Variables|Components|GetBP_PatrolComp)))

(fn RequestTalk
  (params (request_owner :type Actor%20Object%20Reference))
  (bind _result (Default|RequestTalk (Variables|Default|GetBP_CommunicationComp) request_owner))
  (return _result))

(fn SetMoveSpeed
  (params (E_move_speed :type E_MoveSpeed%20Enum :default "NewEnumerator2"))
  (bind _returnvalue (Utilities|GetDataTableRow "/Game/Blueprints/Data/DT_MovementValues.DT_MovementValues" "Default")
    (:then
      (bind _output_get (Variables|/Script/Engine.CharacterMovementComponent|SetMaxWalkSpeed (Variables|Character|GetCharacterMovement) (Utilities|Select :Index E_move_speed :NewEnumerator2 (.Idle_Speed (Utilities|Struct|BreakS_MovementValues _returnvalue)) :NewEnumerator1 (.Walk_Speed (Utilities|Struct|BreakS_MovementValues _returnvalue)) :NewEnumerator0 (.Run_Speed (Utilities|Struct|BreakS_MovementValues _returnvalue)))))
      (return _output_get))
    (:RowNotFound
      (bind _output_get_2 (Variables|/Script/Engine.CharacterMovementComponent|SetMaxWalkSpeed (Variables|Character|GetCharacterMovement) 0.0))
      (return _output_get_2))))